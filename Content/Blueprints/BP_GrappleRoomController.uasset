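; Room controller for a two-wave skeleton ambush that rewards the grapple item.
; When the player overlaps the trigger, it closes the door, waits briefly, then spawns wave one AI from preset transforms.
; Tick polls the spawned enemies, starting wave two, then opening the door, spawning the pickup with a chime and recording itself in the save object's collected pickups.
; The player dog's death event destroys remaining enemies and deactivates the encounter.
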(event OnComponentBeginOverlap(Trigger)
  (params (OverlappedComponent :type Primitive%20Component%20Object%20Reference) (OtherActor :type Actor%20Object%20Reference) (OtherComp :type Primitive%20Component%20Object%20Reference) (OtherBodyIndex :type Integer) (bFromSweep :type Boolean) (SweepResult :type Hit%20Result%20Structure%20%28by%20ref%29))
  (if (not (Variables|Default|GetBeenActivated))
    (if (not (Variables|Default|GetActivated))
      (if (Actor|ActorHasTag OtherActor "Player")
        (Default|CallCloseDoor)
        (Utilities|FlowControl|Delay 1.0)
        (CallFunction|SpawnWave1)
        (Variables|Default|SetWave 1)
        (Variables|Default|SetActivated true)))))

(event Custom|Event%20DeadReset
  (bind _spawnedenemies (Variables|Default|GetSpawnedEnemies))
  (for _array_element _spawnedenemies
    (Utilities|IsValid _array_element
      (:Is%20Valid
        (Actor|DestroyActor _array_element))))
  (Utilities|Array|Clear _spawnedenemies)
  (Variables|Default|SetActivated false))

(event EventBeginPlay
  (bind _asbp_dog (Utilities|Casting|CastToBP_Dog (Game|Player|GetPlayerPawn 0)))
  (EventDispatchers|BindEventtoDead _asbp_dog (delegate Custom|Event%20DeadReset)))

(event EventTick
  (params (DeltaSeconds :type Float%20%28single-precision%29))
  (if (Variables|Default|GetActivated)
    (Variables|Default|SetDeadFlag true)
    (bind _array_element (Utilities|Array|ForEachLoopwithBreak (Variables|Default|GetSpawnedEnemies) :!label _label)
      (:LoopBody
        (if (Utilities|IsValid _array_element)
          (Variables|Default|SetDeadFlag false)
          (goto _label Break)))
      (:Completed
        (if (Variables|Default|GetDeadFlag)
          (if (== (Variables|Default|GetWave) 1)
            (if true
              (CallFunction|SpawnWave2)
              (Variables|Default|SetWave 2))
            (elif (== (Variables|Default|GetWave) 2)
              (if true
                (Default|CallOpenDoor)
                (Game|SpawnActorfromClass "/Game/Blueprints/BP_GrappleItem.BP_GrappleItem_C" (Math|Transform|MakeTransform "950.000000,1950.000000,200.000000" "0, 0, 0" "1.000000,1.000000,1.000000") "Undefined" 0 0)
                (Audio|PlaySoundatLocation "/Game/Sounds/ding-dong_Cue.ding-dong_Cue" "950.000000,1950.000000,200.000000" "0, 0, 0" 1.0 1.0 0.0 0 0 0 0)
                (Variables|Default|SetActivated false)
                (Variables|Default|SetBeenActivated true)
                (bind _asbp_top_down_controller (Utilities|Casting|CastToBP_TopDownController (Game|GetPlayerController 0)))
                (Utilities|Array|AddUnique (Variables|/Game/TopDown/Blueprints/BP_LevelSaveObj.BP_LevelSaveObj_C|GetCollectedPickups (Variables|/Game/TopDown/Blueprints/BP_TopDownGameMode.BP_TopDownGameMode_C|GetLevelSaveObj (Variables|/Game/TopDown/Blueprints/BP_TopDownController.BP_TopDownController_C|GetGameModeRef _asbp_top_down_controller))) self)))))))))

(fn ConstructionScript)

(fn SpawnWave1
  (for _array_element (Variables|Default|GetWave1Transform)
    (bind _returnvalue (AI|SpawnAIFromClass "/Game/Blueprints/BP_Skeleton.BP_Skeleton_C" "/Game/Blueprints/BT_Skeleton.BT_Skeleton" (.location _array_element) (.rotation _array_element) false 0))
    (Utilities|Array|Add (Variables|Default|GetSpawnedEnemies) _returnvalue)))

(fn SpawnWave2
  (for _array_element (Variables|Default|GetWave2Transform)
    (bind _returnvalue (AI|SpawnAIFromClass "/Game/Blueprints/BP_Skeleton.BP_Skeleton_C" "/Game/Blueprints/BT_Skeleton.BT_Skeleton" (.location _array_element) (.rotation _array_element) false 0))
    (Utilities|Array|Add (Variables|Default|GetSpawnedEnemies) _returnvalue)))