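; Two-position lever that the player flips with the context interact input from BP_TopDownController while inside its InteractRange.
; Overlap with a Player-tagged actor enables interaction and turns on custom depth for the lever and base meshes.
; Interacting plays a sound and enables Tick, which rolls the lever to the opposite MaxAngle limit, calls Left or Right, then disables Tick.
; The construction script sets the starting side from IsDefaultLeft.
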(event OnComponentBeginOverlap(InteractRange)
  (params (OverlappedComponent :type Primitive%20Component%20Object%20Reference) (OtherActor :type Actor%20Object%20Reference) (OtherComp :type Primitive%20Component%20Object%20Reference) (OtherBodyIndex :type Integer) (bFromSweep :type Boolean) (SweepResult :type Hit%20Result%20Structure%20%28by%20ref%29))
  (if (Actor|ActorHasTag OtherActor "Player")
    (Variables|Default|SetIsInRange true)
    (Rendering|SetRenderCustomDepth (Variables|Default|GetLever) true)
    (Rendering|SetRenderCustomDepth (Variables|Default|GetBaseMesh) true)))

(event OnComponentEndOverlap(InteractRange)
  (params (OverlappedComponent :type Primitive%20Component%20Object%20Reference) (OtherActor :type Actor%20Object%20Reference) (OtherComp :type Primitive%20Component%20Object%20Reference) (OtherBodyIndex :type Integer))
  (if (Actor|ActorHasTag OtherActor "Player")
    (Variables|Default|SetIsInRange false)
    (Rendering|SetRenderCustomDepth (Variables|Default|GetLever) false)
    (Rendering|SetRenderCustomDepth (Variables|Default|GetBaseMesh) false)))

(event Custom|Event%20Interact
  (bind _speed (Variables|Default|GetSpeed))
  (if (Variables|Default|GetIsInRange)
    (if (not (Variables|Default|GetIsMoving))
      (Variables|Default|SetIsMoving true)
      (Audio|PlaySoundatLocation "/Game/Sounds/switch_sound_Cue.switch_sound_Cue" (Transformation|GetActorLocation) "0, 0, 0" 1.0 1.0 0.0 0 0 0 0)
      (if (> (.roll (Variables|/Script/Engine.SceneComponent|GetRelativeRotation (Variables|Default|GetLever))) 0.0)
        (Variables|Default|SetDirection (* _speed -1.0))
        (Actor|Tick|SetActorTickEnabled true)
        (else
          (Variables|Default|SetDirection _speed)
          (Actor|Tick|SetActorTickEnabled true))))))

(event EventTick
  (params (DeltaSeconds :type Float%20%28single-precision%29))
  (bind _direction (Variables|Default|GetDirection))
  (bind _lever (Variables|Default|GetLever))
  (bind _maxangle (Variables|Default|GetMaxAngle))
  (bind _maxangle_2 (Variables|Default|GetMaxAngle))
  (bind _lever_2 (Variables|Default|GetLever))
  (bind _returnvalue (* _direction DeltaSeconds))
  (bind _returnvalue_2 (* _maxangle -1.0))
  (bind _relativerotation (Variables|/Script/Engine.SceneComponent|GetRelativeRotation _lever_2))
  (bind _returnvalue_3 (+ _returnvalue (.roll _relativerotation)))
  (if (and (< _returnvalue_3 _returnvalue_2) (< _direction 0.0))
    (Transformation|SetRelativeRotation _lever (Math|Rotator|MakeRotator _returnvalue_2 0.0 0.0) false false)
    (Variables|Default|SetIsMoving false)
    (Default|CallLeft)
    (Actor|Tick|SetActorTickEnabled false)
    (elif (and (> _returnvalue_3 _maxangle_2) (> _direction 0.0))
      (Transformation|SetRelativeRotation _lever (Math|Rotator|MakeRotator _maxangle_2 0.0 0.0) false false)
      (Variables|Default|SetIsMoving false)
      (Default|CallRight)
      (Actor|Tick|SetActorTickEnabled false)
      (else
        (Transformation|SetRelativeRotation _lever (Math|Rotator|MakeRotator _returnvalue_3 0.0 0.0) false false)))))

(event EventBeginPlay
  (bind _asbp_top_down_controller (Utilities|Casting|CastToBP_TopDownController (Game|GetPlayerController 0)))
  (EventDispatchers|BindEventtoContextInteract _asbp_top_down_controller (delegate Custom|Event%20Interact)))

(fn ConstructionScript
  (bind _maxangle (Variables|Default|GetMaxAngle))
  (if (Variables|Default|GetIsDefaultLeft)
    (CallFunction|UpdateAngle (* _maxangle -1.0))
    (else
      (CallFunction|UpdateAngle _maxangle))))

(fn UpdateAngle
  (params (Angle :type Float%20%28double-precision%29))
  (Transformation|SetRelativeRotation (Variables|Default|GetLever) (Math|Rotator|MakeRotator Angle 0.0 0.0) false false))