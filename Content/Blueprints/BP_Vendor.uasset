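; Vendor actor that sells the player a rocket for coins, triggered by the top-down controller's context interact event while in range.
; Player overlap highlights the tent via custom depth, shows coin and rocket counts, and flags the controller as at the vendor.
; Tick slides an animated skeleton hand between clamped Y limits on entry and exit.
; Exit resets only once no BP_Dog remains in range.
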(event OnComponentBeginOverlap(InteractRange)
  (params (OverlappedComponent :type Primitive%20Component%20Object%20Reference) (OtherActor :type Actor%20Object%20Reference) (OtherComp :type Primitive%20Component%20Object%20Reference) (OtherBodyIndex :type Integer) (bFromSweep :type Boolean) (SweepResult :type Hit%20Result%20Structure%20%28by%20ref%29))
  (bind _controllerref (Variables|Default|GetControllerRef))
  (if (Actor|ActorHasTag OtherActor "Player")
    (Variables|Default|SetIsInRange true)
    (Rendering|SetRenderCustomDepth (Variables|Default|GetTent) true)
    (Default|CallShowCoinCount _controllerref)
    (Default|CallShowRocketCount _controllerref)
    (Variables|Default|SetIsMoving true)
    (Variables|Default|SetDirection (* (Variables|Default|GetSpeed) -1.0))
    (Components|Animation|PlayAnimation (Variables|Default|GetSkeletonHand) "/Game/Animations/A_SkeletonHandOpen.A_SkeletonHandOpen" false)
    (Variables|/Game/TopDown/Blueprints/BP_TopDownController.BP_TopDownController_C|SetIsAtVendor (Variables|Default|GetControllerRef) true)))

(event OnComponentEndOverlap(InteractRange)
  (params (OverlappedComponent :type Primitive%20Component%20Object%20Reference) (OtherActor :type Actor%20Object%20Reference) (OtherComp :type Primitive%20Component%20Object%20Reference) (OtherBodyIndex :type Integer))
  (bind _controllerref (Variables|Default|GetControllerRef))
  (bind _skeletonhand (Variables|Default|GetSkeletonHand))
  (if (Actor|ActorHasTag OtherActor "Player")
    (if (Utilities|Array|IsEmpty (Collision|GetOverlappingActors (Variables|Default|GetInteractRange) "/Game/Blueprints/BP_Dog.BP_Dog_C" :!class /Script/Engine.PrimitiveComponent))
      (Variables|Default|SetIsInRange false)
      (Rendering|SetRenderCustomDepth (Variables|Default|GetTent) false)
      (Default|CallHideCoinCount _controllerref)
      (Default|CallHideRocketCount _controllerref)
      (Variables|Default|SetIsMoving true)
      (Variables|Default|SetDirection (* (Variables|Default|GetSpeed) 1.0))
      (Components|Animation|PlayAnimation _skeletonhand "/Game/Animations/A_SkeletonHandClose.A_SkeletonHandClose" false)
      (Components|Animation|SetPosition _skeletonhand 1.25 false)
      (Variables|/Game/TopDown/Blueprints/BP_TopDownController.BP_TopDownController_C|SetIsAtVendor (Variables|Default|GetControllerRef) false))))

(event Custom|Event%20TryBuy
  (bind _price (Variables|Default|GetPrice))
  (bind _controllerref (Variables|Default|GetControllerRef))
  (if (Variables|Default|GetIsInRange)
    (if (>= (Variables|/Game/TopDown/Blueprints/BP_TopDownController.BP_TopDownController_C|GetCoins _controllerref) _price)
      (Variables|/Game/TopDown/Blueprints/BP_TopDownController.BP_TopDownController_C|SetCoins _controllerref (- (Variables|/Game/TopDown/Blueprints/BP_TopDownController.BP_TopDownController_C|GetCoins _controllerref) _price))
      (Variables|/Game/TopDown/Blueprints/BP_TopDownController.BP_TopDownController_C|SetRockets _controllerref (+ (Variables|/Game/TopDown/Blueprints/BP_TopDownController.BP_TopDownController_C|GetRockets _controllerref) 1))
      (Audio|PlaySoundatLocation "/Game/Sounds/cha-ching_Cue.cha-ching_Cue" (Transformation|GetActorLocation) "0, 0, 0" 1.0 1.0 0.0 0 0 0 0))))

(event EventBeginPlay
  (bind _asbp_top_down_controller (Utilities|Casting|CastToBP_TopDownController (Game|GetPlayerController 0)))
  (bind _output_get (Variables|Default|SetControllerRef _asbp_top_down_controller))
  (EventDispatchers|BindEventtoContextInteract _output_get (delegate Custom|Event%20TryBuy)))

(event EventTick
  (params (DeltaSeconds :type Float%20%28single-precision%29))
  (bind _skeletonhand (Variables|Default|GetSkeletonHand))
  (bind _skeletonhand_2 (Variables|Default|GetSkeletonHand))
  (bind _direction (Variables|Default|GetDirection))
  (bind _direction_2 (Variables|Default|GetDirection))
  (bind _returnvalue (* DeltaSeconds _direction))
  (bind _relativelocation (Variables|/Script/Engine.SceneComponent|GetRelativeLocation _skeletonhand))
  (bind _relativelocation_2 (Variables|/Script/Engine.SceneComponent|GetRelativeLocation _skeletonhand_2))
  (bind _returnvalue_2 (+ (.y _relativelocation) _returnvalue))
  (if (Variables|Default|GetIsMoving)
    (if (and (< _direction_2 0.0) (< _returnvalue_2 (Variables|Default|GetMinY)))
      (Transformation|SetRelativeLocation _skeletonhand_2 (Math|Vector|MakeVector (.x _relativelocation_2) (Variables|Default|GetMinY) (.z _relativelocation_2)) false false)
      (Variables|Default|SetIsMoving false)
      (elif (and (> _direction_2 0.0) (> _returnvalue_2 (Variables|Default|GetMaxY)))
        (Transformation|SetRelativeLocation _skeletonhand_2 (Math|Vector|MakeVector (.x _relativelocation_2) (Variables|Default|GetMaxY) (.z _relativelocation_2)) false false)
        (Variables|Default|SetIsMoving false)
        (else
          (Transformation|SetRelativeLocation _skeletonhand_2 (Math|Vector|MakeVector (.x _relativelocation_2) _returnvalue_2 (.z _relativelocation_2)) false false))))))

(fn ConstructionScript)