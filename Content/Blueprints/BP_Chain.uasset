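; Chain actor built from instanced mesh segments that appears to be pulled along while a linked drawbridge operates.
; The construction script lays out segments from Length and SegmentLength.
; Movement starts when the linked destructible chain is hit, or on a double drawbridge's Started event with a sound, and stops on Done.
; Tick, toggled with movement, slides instances upward and replaces those beyond half Length with new ones at the origin.
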(event Custom|Event%20Hit
  (if (not (Variables|Default|GetIsWaitingForStarted))
    (Variables|Default|SetIsMoving true)
    (Actor|Tick|SetActorTickEnabled true)))

(event Custom|Event%20Done
  (Variables|Default|SetIsMoving false)
  (Actor|Tick|SetActorTickEnabled false))

(event Custom|Event%20OnStarted
  (if (Variables|Default|GetIsWaitingForStarted)
    (Variables|Default|SetIsMoving true)
    (Actor|Tick|SetActorTickEnabled true)
    (Audio|PlaySoundatLocation "/Game/Sounds/chain-pull_Cue.chain-pull_Cue" (Transformation|GetActorLocation) "0, 0, 0" 1.0 1.0 0.0 0 0 0 0)))

(event EventBeginPlay
  (bind _donedispatcher (Variables|Default|GetDoneDispatcher))
  (bind _asbp_destructible_chain (Utilities|Casting|CastToBP_DestructibleChain (Variables|Default|GetHitDispatcher)))
  (EventDispatchers|BindEventtoHit _asbp_destructible_chain (delegate Custom|Event%20Hit))
  (bind _asbp_drawbridge (Utilities|Casting|CastToBP_Drawbridge _donedispatcher)
    (:then
      (EventDispatchers|BindEventtoDone _asbp_drawbridge (delegate Custom|Event%20Done)))
    (:CastFailed
      (bind _asbp_double_drawbridge (Utilities|Casting|CastToBP_DoubleDrawbridge _donedispatcher))
      (EventDispatchers|BindEventtoDone _asbp_double_drawbridge (delegate Custom|Event%20Done))
      (Variables|Default|SetIsWaitingForStarted true)
      (EventDispatchers|BindEventtoStarted _asbp_double_drawbridge (delegate Custom|Event%20OnStarted)))))

(event EventTick
  (params (DeltaSeconds :type Float%20%28single-precision%29))
  (bind _instancedstaticmesh (Variables|Default|GetInstancedStaticMesh))
  (bind _instancedstaticmesh_2 (Variables|Default|GetInstancedStaticMesh))
  (bind _returnvalue (Components|InstancedStaticMesh|GetInstanceCount _instancedstaticmesh))
  (bind _returnvalue_2 (- _returnvalue 1))
  (if (Variables|Default|GetIsMoving)
    (for _index (range 0 _returnvalue_2)
      (Components|InstancedStaticMesh|UpdateInstanceTransform _instancedstaticmesh _index (Math|Transform|MakeTransform (+ (.Location (Math|Transform|BreakTransform (.OutInstanceTransform (Components|InstancedStaticMesh|GetInstanceTransform _instancedstaticmesh _index false)))) (* (Math|Vector|VectorUp) (* DeltaSeconds (Variables|Default|GetMoveSpeed)))) (.Rotation (Math|Transform|BreakTransform (.OutInstanceTransform (Components|InstancedStaticMesh|GetInstanceTransform _instancedstaticmesh _index false)))) (.Scale (Math|Transform|BreakTransform (.OutInstanceTransform (Components|InstancedStaticMesh|GetInstanceTransform _instancedstaticmesh _index false))))) false (== _index _returnvalue_2) false)
      (if (> (Math|Vector|VectorLength (+ (.Location (Math|Transform|BreakTransform (.OutInstanceTransform (Components|InstancedStaticMesh|GetInstanceTransform _instancedstaticmesh _index false)))) (* (Math|Vector|VectorUp) (* DeltaSeconds (Variables|Default|GetMoveSpeed))))) (/ (Variables|Default|GetLength) 2.0))
        (Class|InstancedStaticMeshComponent|RemoveInstance _instancedstaticmesh_2 _index)
        (Components|InstancedStaticMesh|AddInstance _instancedstaticmesh_2 (Math|Conversions|ToTransform(Vector) (Math|Vector|VectorZero)) false)))))

(fn ConstructionScript
  (CallFunction|UpdateLength))

(fn UpdateLength
  (bind _length (Variables|Default|GetLength))
  (bind _segmentlength (Variables|Default|GetSegmentLength))
  (bind _returnvalue (/ _length _segmentlength))
  (bind _returnvalue_2 (Math|Float|Ceil _returnvalue))
  (if (not (== (Variables|Default|GetSegments) _returnvalue_2))
    (Components|InstancedStaticMesh|ClearInstances (Variables|Default|GetInstancedStaticMesh))
    (bind _output_get (Variables|Default|SetSegments _returnvalue_2))
    (for _index (range 0 (- _output_get 1))
      (Components|InstancedStaticMesh|AddInstance (Variables|Default|GetInstancedStaticMesh) (Math|Conversions|ToTransform(Vector) (* (* (Math|Vector|VectorUp) (/ (Variables|Default|GetSegmentLength) 2.0)) _index)) false))))