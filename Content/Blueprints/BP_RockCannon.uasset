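; BP_RockCannon is a boss-battle cannon that turns toward the player and fires BP_ProjectileRock projectiles.
; Boss controller start and reset signals activate or deactivate it, and Tick yaws the base and barrel toward the player while active.
; LaunchProjectile spawns a rock along the barrel's forward vector and re-arms itself by timer after an initial delay.
; Death hides the meshes, stops firing and spawns a poof.
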(event Custom|Event%20Start
  (CallFunction|Activate))

(event Custom|Event%20Reset
  (CallFunction|Deactivate))

(event EventBeginPlay
  (bind _bosscontroller (Variables|Default|GetBossController))
  (|CallParentFunction)
  (if (Variables|Default|GetIsActive)
    (CallFunction|Activate))
  (EventDispatchers|BindEventtoBattleStartSignal _bosscontroller (delegate Custom|Event%20Start))
  (EventDispatchers|BindEventtoBattleResetSignal _bosscontroller (delegate Custom|Event%20Reset)))

(event EventTick
  (params (DeltaSeconds :type Float%20%28single-precision%29))
  (bind _returnvalue (Game|Player|GetPlayerPawn 0))
  (bind _cannonmesh (Variables|Default|GetCannonMesh))
  (bind _returnvalue_2 (Transformation|GetActorLocation _returnvalue))
  (bind _returnvalue_3 (Transformation|GetWorldLocation _cannonmesh))
  (bind _returnvalue_4 (Math|Rotator|FindLookatRotation _returnvalue_3 _returnvalue_2))
  (bind (_roll _pitch _yaw) (Math|Rotator|BreakRotator _returnvalue_4))
  (if (Variables|Default|GetIsActive)
    (Transformation|SetWorldRotation (Variables|Default|GetRotatingBaseMesh) (Math|Rotator|MakeRotator 0.0 0.0 _yaw) false false)
    (Transformation|SetWorldRotation (Variables|Default|GetCannonMesh) (Math|Rotator|MakeRotator _roll 0.0 _yaw) false false)))

(fn ConstructionScript
  (|CallParentFunction))

(fn LaunchProjectile
  (bind _cannonmesh (Variables|Default|GetCannonMesh))
  (bind _returnvalue (Transformation|GetWorldTransform _cannonmesh))
  (bind _returnvalue_2 (Game|SpawnActorfromClass "/Game/Blueprints/BP_ProjectileRock.BP_ProjectileRock_C" (Math|Transform|MakeTransform (+ (.location _returnvalue) (Variables|Default|GetLaunchOffset)) (.rotation _returnvalue) "1.000000,1.000000,1.000000") "Undefined" 0 0))
  (Variables|/Game/Blueprints/BP_ProjectileRock.BP_ProjectileRock_C|SetDirection _returnvalue_2 (Math|Vector|GetForwardVector _cannonmesh))
  (if (Variables|Default|GetIsActive)
    (Utilities|Time|SetTimerbyFunctionName 0 "LaunchProjectile" (Variables|Default|GetFireDelay))))

(fn Activate
  (CallFunction|SetVisible true)
  (Variables|Default|SetIsActive true)
  (Utilities|Time|SetTimerbyFunctionName 0 "LaunchProjectile" (Variables|Default|GetFireInitialOffset)))

(fn Deactivate
  (Variables|Default|SetIsActive false)
  (Utilities|Time|ClearTimerbyFunctionName 0 "LaunchProjectile")
  (Transformation|SetRelativeRotation (Variables|Default|GetRotatingBaseMesh) "0, 0, 0" false false)
  (Transformation|SetRelativeRotation (Variables|Default|GetCannonMesh) "0, 0, 0" false false))

(fn Death
  (CallFunction|SetVisible false)
  (CallFunction|Deactivate)
  (Game|SpawnActorfromClass "/Game/Blueprints/BP_Poof.BP_Poof_C" (Transformation|GetActorTransform) "Undefined" 0 0))

(fn SetVisible
  (params (Visibility :type Boolean))
  (Rendering|SetVisibility (Variables|Default|GetStaticBaseMesh) Visibility false)
  (Rendering|SetVisibility (Variables|Default|GetRotatingBaseMesh) Visibility false)
  (Rendering|SetVisibility (Variables|Default|GetCannonMesh) Visibility false)
  (Rendering|SetVisibility (Variables|Default|GetBlackoutPlaneMesh) Visibility false))