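; BP_ProjectileRock is a rock projectile that damages dogs and enemies on impact.
; Tick moves it along Direction at Speed without sweeping, relying on DamageSphere overlaps for hits.
; After a brief invincible window at spawn, any overlap spawns an explosion and applies Damage to a BP_Dog or BP_Enemy.
; The rock then destroys itself, except on Cannon-tagged actors, where it explodes but survives undamaging.
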(event OnComponentBeginOverlap(DamageSphere)
  (params (OverlappedComponent :type Primitive%20Component%20Object%20Reference) (OtherActor :type Actor%20Object%20Reference) (OtherComp :type Primitive%20Component%20Object%20Reference) (OtherBodyIndex :type Integer) (bFromSweep :type Boolean) (SweepResult :type Hit%20Result%20Structure%20%28by%20ref%29))
  (if (not (Variables|Default|GetInvincible))
    (Game|SpawnActorfromClass "/Game/Blueprints/BP_ProjectileExplosion.BP_ProjectileExplosion_C" (Transformation|GetActorTransform) "Undefined" 0 0)
    (if (Utilities|IsValid OtherActor)
      (if (not (Actor|ActorHasTag OtherActor "Cannon"))
        (bind _asbp_dog (Utilities|Casting|CastToBP_Dog OtherActor)
          (:then
            (Default|DamageDog _asbp_dog (Variables|Default|GetDamage)))
          (:CastFailed
            (bind _asbp_enemy (Utilities|Casting|CastToBP_Enemy OtherActor)
              (:then
                (Default|DamageEnemy _asbp_enemy (Variables|Default|GetDamage)))
              (:CastFailed
                _))))
        (Actor|DestroyActor :!label _label))
      (else
        (goto _label)))))

(event EventTick
  (params (DeltaSeconds :type Float%20%28single-precision%29))
  (Transformation|SetActorLocation (+ (Transformation|GetActorLocation) (* (Variables|Default|GetDirection) (Variables|Default|GetSpeed) DeltaSeconds)) false false))

(event EventBeginPlay
  (Variables|Default|SetInvincible true)
  (Utilities|FlowControl|Delay 0.2)
  (Variables|Default|SetInvincible false))

(fn ConstructionScript)