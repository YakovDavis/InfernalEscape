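; BP_Rocket is a firework rocket projectile that flies along a set direction and deals explosive damage to enemies.
; Tick moves it without sweep, and a brief invincibility window after spawn keeps it from detonating immediately.
; A trigger sphere overlap with any non-Player actor damages every BP_Enemy inside a separate damage sphere and calls Boom.
; It then stops, swaps engine effects and whistle for explosion effects, and destroys itself after a delay.
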(event OnComponentBeginOverlap(TriggerSphere)
  (params (OverlappedComponent :type Primitive%20Component%20Object%20Reference) (OtherActor :type Actor%20Object%20Reference) (OtherComp :type Primitive%20Component%20Object%20Reference) (OtherBodyIndex :type Integer) (bFromSweep :type Boolean) (SweepResult :type Hit%20Result%20Structure%20%28by%20ref%29))
  (if (Variables|Default|GetIsMoving)
    (if (not (Variables|Default|GetIsInvincible))
      (if (not (Actor|ActorHasTag OtherActor "Player"))
        (for _array_element (Collision|GetOverlappingActors (Variables|Default|GetDamageSphere) "/Game/Blueprints/BP_Enemy.BP_Enemy_C" :!class /Script/Engine.PrimitiveComponent)
          (bind _asbp_enemy (Utilities|Casting|CastToBP_Enemy _array_element))
          (Default|ExplosiveDamageEnemy _asbp_enemy (Variables|Default|GetDamage)))
        (Default|CallBoom)
        (Variables|Default|SetIsMoving false)
        (Components|Activation|Activate (Variables|Default|GetExplosionNS) false)
        (Rendering|SetVisibility (Variables|Default|GetStaticMesh) false false)
        (Components|Activation|Deactivate (Variables|Default|GetEngineNS))
        (Audio|Components|Audio|Stop (Variables|Default|GetWhistleSound))
        (Audio|PlaySoundatLocation "/Game/Sounds/fireworks-explosion_Cue.fireworks-explosion_Cue" (Transformation|GetActorLocation) "0, 0, 0" 1.0 1.0 0.0 0 0 0 0)
        (Utilities|FlowControl|Delay 1.0)
        (Actor|DestroyActor)))))

(event EventTick
  (params (DeltaSeconds :type Float%20%28single-precision%29))
  (if (Variables|Default|GetIsMoving)
    (Transformation|SetActorLocation (+ (Transformation|GetActorLocation) (* (Variables|Default|GetDirection) (Variables|Default|GetSpeed) DeltaSeconds)) false false)))

(event EventBeginPlay
  (Audio|PlaySoundatLocation "/Game/Sounds/firework-launch_Cue.firework-launch_Cue" "0, 0, 0" "0, 0, 0" 1.0 1.0 0.0 0 0 0 0)
  (Variables|Default|SetIsInvincible true)
  (Utilities|FlowControl|Delay 0.2)
  (Variables|Default|SetIsInvincible false)
  (bind _returnvalue (Audio|SpawnSoundatLocation "/Game/Sounds/firework-whistle_Cue.firework-whistle_Cue" (Transformation|GetActorLocation) "0, 0, 0" 1.0 1.0 0.0 0 0))
  (Variables|Default|SetWhistleSound _returnvalue))

(fn ConstructionScript)