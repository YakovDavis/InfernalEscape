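; Skeleton enemy that fights the dog, extending a parent enemy class with its own attack, hit feedback and death.
; Attack briefly arms the weapon collision, which damages BP_Dog at most once per swing.
; Normal and explosive damage play a smash sound, flash red through a dynamic material and call WasAttacked.
; Death randomly drops health and coins, then leaves either a bone pile inheriting its patrol radius or a poof.
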(event OnComponentBeginOverlap(WeaponCollision)
  (params (OverlappedComponent :type Primitive%20Component%20Object%20Reference) (OtherActor :type Actor%20Object%20Reference) (OtherComp :type Primitive%20Component%20Object%20Reference) (OtherBodyIndex :type Integer) (bFromSweep :type Boolean) (SweepResult :type Hit%20Result%20Structure%20%28by%20ref%29))
  (if (Variables|Default|GetIsWeaponDamaging)
    (bind _asbp_dog (Utilities|Casting|CastToBP_Dog OtherActor))
    (if (not (Variables|Default|GetHitConnected))
      (Default|DamageDog _asbp_dog 0.5)
      (Variables|Default|SetHitConnected true))))

(event Custom|DmgIndicate
  (bind _mi (Variables|Default|GetMI))
  (Rendering|Material|SetScalarParameterValue _mi "DMG Red" 1.0 :!class /Script/Engine.MaterialInstanceDynamic)
  (Utilities|FlowControl|Delay 0.2)
  (Rendering|Material|SetScalarParameterValue _mi "DMG Red" 0.0 :!class /Script/Engine.MaterialInstanceDynamic))

(event Custom|Event%20Attack
  (Variables|Default|SetHitConnected false)
  (Variables|Default|SetIsWeaponDamaging true)
  (Utilities|FlowControl|Delay 0.2)
  (Variables|Default|SetIsWeaponDamaging false))

(event EventBeginPlay
  (|CallParentFunction)
  (bind _returnvalue (Rendering|Material|CreateDynamicMaterialInstance "/Game/Materials/M_Esqueleto.M_Esqueleto" "None" "None" :!class /Script/Engine.KismetMaterialLibrary))
  (bind _output_get (Variables|Default|SetMI _returnvalue))
  (Rendering|Material|SetMaterial (Variables|Character|GetMesh) 0 _output_get))

(event Collision|EventActorBeginOverlap
  (params (OtherActor :type Actor%20Object%20Reference))
  (|CallParentFunction OtherActor) ; This node is disabled and will not be called.\nDrag off pins to build functionality.
)

(event EventTick
  (params (DeltaSeconds :type Float%20%28single-precision%29))
  (|CallParentFunction DeltaSeconds) ; This node is disabled and will not be called.\nDrag off pins to build functionality.
)

(fn ConstructionScript
  (|CallParentFunction))

(fn DamageEnemy
  (params (Damage :type Float%20%28double-precision%29))
  (|CallParentFunction Damage)
  (Audio|PlaySoundatLocation "/Game/Sounds/skeleton_getting_smashed_Cue.skeleton_getting_smashed_Cue" (Transformation|GetActorLocation) "0, 0, 0" 1.0 1.0 0.0 0 0 0 0)
  (CallFunction|DmgIndicate)
  (Default|CallWasAttacked))

(fn ExplosiveDamageEnemy
  (params (Damage :type Float%20%28double-precision%29))
  (|CallParentFunction Damage)
  (Audio|PlaySoundatLocation "/Game/Sounds/skeleton_getting_smashed_Cue.skeleton_getting_smashed_Cue" (Transformation|GetActorLocation) "0, 0, 0" 1.0 1.0 0.0 0 0 0 0)
  (CallFunction|DmgIndicate)
  (Default|CallWasAttacked))

(fn Death
  (if (Math|Random|RandomBool)
    (Game|SpawnActorfromClass "/Game/Blueprints/BP_HealthPickup.BP_HealthPickup_C" (Math|Transform|MakeTransform (+ (Transformation|GetActorLocation) (* (Math|Random|RandomUnitVectorinConeinDegrees "0.000000, 0,1.000000" 9e+01) (Math|Random|RandomFloatinRange 0.0 5e+01))) "0, 0, 0" "1.000000,1.000000,1.000000") "Undefined" 0 0))
  (if (Math|Random|RandomBool)
    (Game|SpawnActorfromClass "/Game/Blueprints/BP_Coin.BP_Coin_C" (Math|Transform|MakeTransform (+ (Transformation|GetActorLocation) (* (Math|Random|RandomUnitVectorinConeinDegrees "0.000000, 0,1.000000" 9e+01) (Math|Random|RandomFloatinRange 0.0 5e+01))) "0, 0, 0" "1.000000,1.000000,1.000000") "Undefined" 0 0))
  (if (Math|Random|RandomBool)
    (Game|SpawnActorfromClass "/Game/Blueprints/BP_Coin.BP_Coin_C" (Math|Transform|MakeTransform (+ (Transformation|GetActorLocation) (* (Math|Random|RandomUnitVectorinConeinDegrees "0.000000, 0,1.000000" 9e+01) (Math|Random|RandomFloatinRange 0.0 5e+01))) "0, 0, 0" "1.000000,1.000000,1.000000") "Undefined" 0 0))
  (if (Variables|Default|GetLeavesPileOfBones)
    (bind _returnvalue (Game|SpawnActorfromClass "/Game/Blueprints/BP_PileOfBones.BP_PileOfBones_C" (Transformation|GetActorTransform) "Undefined" 0 0))
    (Variables|/Game/Blueprints/BP_PileOfBones.BP_PileOfBones_C|SetPatrolRadius _returnvalue (Variables|Default|GetPatrolRadius))
    (else
      (CallFunction|MakePoof)))
  (Actor|DestroyActor))

(fn MakePoof
  (Game|SpawnActorfromClass "/Game/Blueprints/BP_Poof.BP_Poof_C" (Transformation|GetActorTransform) "Undefined" 0 0))