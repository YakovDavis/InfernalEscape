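; BP_RockPuzzleController runs a rock-moving puzzle that rewards a bone key item when solved.
; It records rock start locations at BeginPlay and restores them when the reset switch is hit.
; Each rock's move event triggers a check that every target location exactly matches some rock's location, in any order.
; Success locks the rocks, spawns the key at a hardcoded position and plays a chime.
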(event Custom|Event%20UpdateStones
  (Variables|Default|SetIsCorrect true)
  (Utilities|Set|Clear (Variables|Default|GetLocationsSet))
  (for _array_element (Variables|Default|GetRocks)
    (Utilities|Set|Add (Variables|Default|GetLocationsSet) (Transformation|GetActorLocation _array_element)))
  (bind _array_element_2 (Utilities|Array|ForEachLoopwithBreak (Variables|Default|GetTargetsSet) :!label _label)
    (:LoopBody
      (if (not (Utilities|Set|Contains (Variables|Default|GetLocationsSet) _array_element_2))
        (Variables|Default|SetIsCorrect false)
        (goto _label Break)))
    (:Completed
      (if (Variables|Default|GetIsCorrect)
        (for _array_element_3 (Variables|Default|GetRocks)
          (Variables|/Game/Blueprints/BP_MovableRock.BP_MovableRock_C|SetCanMoveNow _array_element_3 false))
        (Game|SpawnActorfromClass "/Game/Blueprints/BP_BoneKeyItem.BP_BoneKeyItem_C" (Math|Transform|MakeTransform "5460.000000,-550.000000,240.000000" "0, 0, 0" "1.000000,1.000000,1.000000") "Undefined" 0 0)
        (Audio|PlaySoundatLocation "/Game/Sounds/ding-dong_Cue.ding-dong_Cue" "5460.000000,-550.000000,200.000000" "0, 0, 0" 1.0 1.0 0.0 0 0 0 0)))))

(event Custom|Event%20ResetPuzzle
  (for (_array_element _array_index) (Variables|Default|GetRocks)
    (Transformation|SetActorLocation _array_element (Utilities|Array|Get(acopy) (Variables|Default|GetInitLocationsSet) _array_index) false false)))

(event EventBeginPlay
  (bind _rocks (Variables|Default|GetRocks))
  (for (_array_element _array_index) _rocks
    (EventDispatchers|BindEventtoHeyIveMoved _array_element (delegate Custom|Event%20UpdateStones))
    (Utilities|Array|Add (Variables|Default|GetInitLocationsSet) (Transformation|GetActorLocation (Utilities|Array|Get(acopy) _rocks _array_index))))
  (EventDispatchers|BindEventtoHit (Variables|Default|GetResetSwitch) (delegate Custom|Event%20ResetPuzzle)))

(fn ConstructionScript)