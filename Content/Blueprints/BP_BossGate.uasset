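; BP_BossGate is a double gate that closes when a boss battle starts and opens when the battle resets or its lock is unlocked.
; On BeginPlay it binds those responses to signals from a boss controller and a lock reference.
; Tick swings the two meshes in mirrored yaw at a set speed, clamping at closed or the open angle.
; The construction script can pose it open by default.
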(event Custom|Event%20BattleStart
  (Variables|Default|SetIsMoving true)
  (Variables|Default|SetDirection (* (Variables|Default|GetSpeed) -1.0)))

(event Custom|Event%20BattleReset
  (Variables|Default|SetIsMoving true)
  (Variables|Default|SetDirection (Variables|Default|GetSpeed)))

(event Custom|Event%20Open
  (Variables|Default|SetIsMoving true)
  (Variables|Default|SetDirection (Variables|Default|GetSpeed)))

(event EventTick
  (params (DeltaSeconds :type Float%20%28single-precision%29))
  (bind _direction (Variables|Default|GetDirection))
  (bind _leftmesh (Variables|Default|GetLeftMesh))
  (bind _direction_2 (Variables|Default|GetDirection))
  (bind _returnvalue (* DeltaSeconds _direction))
  (bind _relativerotation (Variables|/Script/Engine.SceneComponent|GetRelativeRotation _leftmesh))
  (bind _returnvalue_2 (+ (.yaw _relativerotation) _returnvalue))
  (if (Variables|Default|GetIsMoving)
    (if (and (< _direction_2 0.0) (< _returnvalue_2 0.0))
      (CallFunction|UpdateAngle 0.0)
      (Variables|Default|SetIsMoving false)
      (elif (and (> _direction_2 0.0) (> _returnvalue_2 (Variables|Default|GetOpenAngle)))
        (CallFunction|UpdateAngle (Variables|Default|GetOpenAngle))
        (Variables|Default|SetIsMoving false)
        (else
          (CallFunction|UpdateAngle _returnvalue_2))))))

(event EventBeginPlay
  (bind _bosscontroller (Variables|Default|GetBossController))
  (EventDispatchers|BindEventtoBattleStartSignal _bosscontroller (delegate Custom|Event%20BattleStart))
  (EventDispatchers|BindEventtoBattleResetSignal _bosscontroller (delegate Custom|Event%20BattleReset))
  (EventDispatchers|BindEventtoUnlocked (Variables|Default|GetLockRef) (delegate Custom|Event%20Open)))

(fn ConstructionScript
  (if (Variables|Default|GetDefaultOpen)
    (CallFunction|UpdateAngle (Variables|Default|GetOpenAngle))))

(fn UpdateAngle
  (params (Angle :type Float%20%28double-precision%29))
  (Transformation|SetRelativeRotation (Variables|Default|GetLeftMesh) (Math|Rotator|MakeRotator 0.0 0.0 Angle) false false)
  (Transformation|SetRelativeRotation (Variables|Default|GetRightMesh) (Math|Rotator|MakeRotator 0.0 0.0 (* Angle -1.0)) false false))