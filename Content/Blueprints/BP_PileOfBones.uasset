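; BP_PileOfBones is the remains of a skeleton enemy that revives after a countdown.
; It plays a death sound on spawn, then Tick counts down while active.
; At zero it plays the falling animation in reverse as a rise, with a revive sound.
; A timer then spawns an AI BP_Skeleton in its place, sets its HP and flags it to leave another pile, and destroys itself.
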(event EventBeginPlay
  (Audio|PlaySoundatLocation "/Game/Sounds/skeleton_dying_Cue.skeleton_dying_Cue" (Transformation|GetActorLocation) "0, 0, 0" 1.0 1.0 0.0 0 0 0 0))

(event EventTick
  (params (DeltaSeconds :type Float%20%28single-precision%29))
  (if (Variables|Default|GetIsActive)
    (bind _output_get (Variables|Default|SetTimeRemaining (- (Variables|Default|GetTimeRemaining) DeltaSeconds)))
    (if (<= _output_get 0.0)
      (Components|Animation|PlayAnimation (Variables|Default|GetSkeletalMesh) "/Game/Animations/Skeleton/Skeleton-falling_Anim.Skeleton-falling_Anim" false)
      (Components|Animation|SetPosition (Variables|Default|GetSkeletalMesh) 1.25 false)
      (Components|Timeline|SetPlayRate (Variables|Default|GetSkeletalMesh) -1.0)
      (Audio|PlaySoundatLocation "/Game/Sounds/skeleton_reviving_Cue.skeleton_reviving_Cue" (Transformation|GetActorLocation) "0, 0, 0" 1.0 1.0 0.0 0 0 0 0)
      (Variables|Default|SetIsActive false)
      (Utilities|Time|SetTimerbyFunctionName 0 "SpawnSkeleton" 1.5))))

(fn ConstructionScript)

(fn SpawnSkeleton
  (bind _returnvalue (AI|SpawnAIFromClass "/Game/Blueprints/BP_Skeleton.BP_Skeleton_C" "/Game/Blueprints/BT_Skeleton.BT_Skeleton" (Transformation|GetActorLocation) (Transformation|GetActorRotation) false 0))
  (bind _asbp_skeleton (Utilities|Casting|CastToBP_Skeleton _returnvalue)
    (:then
      (Variables|/Game/Blueprints/BP_Skeleton.BP_Skeleton_C|SetLeavesPileOfBones _asbp_skeleton true)
      (Variables|/Game/Blueprints/BP_Enemy.BP_Enemy_C|SetHP _asbp_skeleton 5.0))
    (:CastFailed
      _))
  (Actor|DestroyActor))