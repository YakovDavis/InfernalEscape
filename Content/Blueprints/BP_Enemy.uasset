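; Enemy Blueprint that takes melee and explosive damage from the player's dog pawn and destroys itself when its health runs out.
; On BeginPlay it caches the player as BP_Dog to read the controller's equipped weapon.
; Per-weapon flags gate stick, club and sword hits, and a disallowed weapon signals the top-down controller to stop attacking.
; Explosive damage has its own flag.
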(event EventBeginPlay
  (bind _asbp_dog (Utilities|Casting|CastToBP_Dog (Game|Player|GetPlayerPawn 0)))
  (Variables|Default|SetPlayerRef _asbp_dog))

(fn ConstructionScript)

(fn DamageEnemy
  (params (Damage :type Float%20%28double-precision%29))
  (bind _playerref (Variables|Default|GetPlayerRef))
  (bind _controllerref (Variables|/Game/Blueprints/BP_Dog.BP_Dog_C|GetControllerRef _playerref))
  (bind _weapon (Variables|/Game/TopDown/Blueprints/BP_TopDownController.BP_TopDownController_C|GetWeapon _controllerref))
  (if (Variables|Default|GetIsAttackable)
    (if (Math|Boolean|ORBoolean (and (== _weapon 0) (Variables|Default|GetIsStickAttackable)) (and (== _weapon 1) (Variables|Default|GetIsClubAttackable)) (and (== _weapon 2) (Variables|Default|GetIsSwordAttackable)))
      (bind _output_get (Variables|Default|SetHP (- (Variables|Default|GetHP) Damage)))
      (if (<= _output_get 0.0)
        (CallFunction|Death))
      (else
        (bind _asbp_top_down_controller (Utilities|Casting|CastToBP_TopDownController (Game|GetPlayerController 0)))
        (Default|SignalStopAttacking _asbp_top_down_controller)))))

(fn Death
  (Actor|DestroyActor))

(fn ExplosiveDamageEnemy
  (params (Damage :type Float%20%28double-precision%29))
  (if (Variables|Default|GetIsAttackable)
    (if (Variables|Default|GetIsExplosiveAttackable)
      (bind _output_get (Variables|Default|SetHP (- (Variables|Default|GetHP) Damage)))
      (if (<= _output_get 0.0)
        (CallFunction|Death)))))