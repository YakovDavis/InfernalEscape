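; BP_Dog is the player's dog character, with melee weapons, blocking, gadgets and heart-based health.
; It binds to BP_TopDownController events for weapon swaps, attacks, blocks and gadget shots, toggling controllability during gadget use and shock.
; Weapon overlaps damage each enemy once per swing, with non-piercing weapons stopping on first hit.
; Tick drives the grapple as shoot, retract or pull states, switched by probe overlaps with "Grappable" actors.
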(event OnComponentBeginOverlap(WeaponCollision)
  (params (OverlappedComponent :type Primitive%20Component%20Object%20Reference) (OtherActor :type Actor%20Object%20Reference) (OtherComp :type Primitive%20Component%20Object%20Reference) (OtherBodyIndex :type Integer) (bFromSweep :type Boolean) (SweepResult :type Hit%20Result%20Structure%20%28by%20ref%29))
  (bind _enemieshit (Variables|Default|GetEnemiesHit))
  (if (Variables|Default|GetIsWeaponDamaging)
    (bind _asbp_enemy (Utilities|Casting|CastToBP_Enemy OtherActor))
    (if (not (Utilities|Set|Contains _enemieshit _asbp_enemy))
      (Default|DamageEnemy _asbp_enemy (Utilities|Array|Get(acopy) (Variables|Default|GetWeaponDmgTable) (Variables|/Game/TopDown/Blueprints/BP_TopDownController.BP_TopDownController_C|GetWeapon (Variables|Default|GetControllerRef))))
      (Utilities|Set|Add _enemieshit _asbp_enemy)
      (if (not (Variables|Default|GetIsWeaponPiercing))
        (Variables|Default|SetIsWeaponDamaging false)
        (Default|SignalStopAttacking (Variables|Default|GetControllerRef))
        (Default|CallAttackInterrupted)))))

(event OnComponentBeginOverlap(GrappleProbe)
  (params (OverlappedComponent :type Primitive%20Component%20Object%20Reference) (OtherActor :type Actor%20Object%20Reference) (OtherComp :type Primitive%20Component%20Object%20Reference) (OtherBodyIndex :type Integer) (bFromSweep :type Boolean) (SweepResult :type Hit%20Result%20Structure%20%28by%20ref%29))
  (if (Variables|Default|GetIsGrappleShooting)
    (if (Actor|ActorHasTag OtherActor "Grappable")
      (Variables|Default|SetIsGrappleShooting false)
      (Variables|Default|SetIsGrappleMoving true)
      (Variables|/Script/Engine.CharacterMovementComponent|SetGravityScale (Variables|Character|GetCharacterMovement) 0.0)
      (Audio|SpawnSoundatLocation "/Game/Sounds/grapple-land_Cue.grapple-land_Cue" (Transformation|GetActorLocation) "0, 0, 0" 1.0 1.0 0.0 0 0)
      (elif (not (Actor|ActorHasTag OtherActor "Player"))
        (Variables|Default|SetIsGrappleShooting false)
        (Variables|Default|SetIsGrappleRetracting true)))))

(event Custom|Event%20UpdateWeapon
  (CallFunction|UpdateWeapon))

(event Custom|Event%20StartAttacking
  (Audio|PlaySoundatLocation "/Game/Sounds/sword_swing_Cue.sword_swing_Cue" (Transformation|GetActorLocation) "0, 0, 0" 1.0 1.0 0.0 0 0 0 0)
  (Variables|Default|SetIsWeaponDamaging true)
  (Variables|Default|SetEnemiesHit (Utilities|Set|MakeSet)))

(event Custom|Event%20AcquirePartOfHeart
  (bind _controllerref (Variables|Default|GetControllerRef))
  (Audio|PlaySoundatLocation "/Game/Sounds/weapon-pickup_Cue.weapon-pickup_Cue" (Transformation|GetActorLocation) "0, 0, 0" 1.0 1.0 0.0 0 0 0 0)
  (if (>= (+ (Variables|Default|GetHeartPartsCollected) 1) 4)
    (CallFunction|EventAcquireHeart)
    (Variables|Default|SetHeartPartsCollected 0)
    (else
      (Variables|Default|SetHeartPartsCollected (+ (Variables|Default|GetHeartPartsCollected) 1))))
  (Default|CallShowBoneCount _controllerref)
  (Utilities|FlowControl|Delay 2.0)
  (Default|CallHideBoneCount _controllerref))

(event Custom|Event%20StopBlock
  (Variables|Default|SetIsBlocking false)
  (Transformation|SetRelativeRotation (Variables|Default|GetWeaponMesh) "0, 0, 0" false false))

(event Custom|Event%20StartBlock
  (Variables|Default|SetIsBlocking true)
  (Transformation|SetRelativeRotation (Variables|Default|GetWeaponMesh) "0, 0,-70.000000" false false))

(event Custom|Event%20GrapplingShot
  (CallFunction|SetControllable false)
  (CallFunction|DisplayGadget)
  (Default|CallStartGrappling)
  (Utilities|FlowControl|Delay 1.0)
  (Variables|Default|SetIsGrappleShooting true)
  (Rendering|SetVisibility (Variables|Default|GetGrappleHook) true false)
  (Rendering|SetVisibility (Variables|Default|GetGrappleRope) true false)
  (Rendering|SetVisibility (Variables|Default|GetGrapplingHookFake) false false))

(event Custom|Event%20RocketLaunch
  (bind _returnvalue (Transformation|GetActorTransform))
  (bind (_location _rotation _scale) (Math|Transform|BreakTransform _returnvalue))
  (CallFunction|SetControllable false)
  (CallFunction|DisplayGadget)
  (Default|CallFireRocket)
  (Utilities|FlowControl|Delay 1.0)
  (bind _returnvalue_2 (Game|SpawnActorfromClass "/Game/Blueprints/BP_Rocket.BP_Rocket_C" (Math|Transform|MakeTransform (+ _location (Math|Vector|MakeVector 4e+01 2e+01 0.0)) _rotation _scale) "Undefined" 0 0))
  (Variables|/Game/Blueprints/BP_Rocket.BP_Rocket_C|SetDirection _returnvalue_2 (Math|Rotator|GetRotationXVector (Transformation|GetActorRotation)))
  (EventDispatchers|BindEventtoBoom _returnvalue_2 (delegate Custom|Event%20Shock))
  (CallFunction|UpdateWeapon)
  (CallFunction|SetControllable true))

(event Custom|Event%20Shock
  (if (Variables|/Game/TopDown/Blueprints/BP_TopDownController.BP_TopDownController_C|GetIsPlayerControllable (Variables|Default|GetControllerRef))
    (Default|CallShocked)
    (CallFunction|SetControllable false)
    (Utilities|FlowControl|Delay 2.0)
    (CallFunction|SetControllable true)))

(event Custom|Event%20AcquireHeart
  (bind _output_get (Variables|Default|SetMaxHP (+ (Variables|Default|GetMaxHP) 1.0)))
  (Variables|Default|SetHP _output_get)
  (Default|CallUpdateHealth)
  (Audio|PlaySoundatLocation "/Game/Sounds/ding-dong_Cue.ding-dong_Cue" (Transformation|GetActorLocation) "0, 0, 0" 1.0 1.0 0.0 0 0 0 0))

(event Custom|Event%20StopAttacking
  (Variables|Default|SetIsWeaponDamaging false))

(event EventBeginPlay
  (bind _asbp_top_down_controller (Utilities|Casting|CastToBP_TopDownController (Pawn|GetController)))
  (bind _output_get (Variables|Default|SetControllerRef _asbp_top_down_controller))
  (EventDispatchers|BindEventtoUpdateWeapon _output_get (delegate Custom|Event%20UpdateWeapon))
  (EventDispatchers|BindEventtoStartAttacking _output_get (delegate Custom|Event%20StartAttacking))
  (EventDispatchers|BindEventtoStopAttacking _output_get (delegate Custom|Event%20StopAttacking))
  (CallFunction|EventUpdateWeapon)
  (EventDispatchers|BindEventtoStartBlocking _asbp_top_down_controller (delegate Custom|Event%20StartBlock))
  (EventDispatchers|BindEventtoStopBlocking _asbp_top_down_controller (delegate Custom|Event%20StopBlock))
  (EventDispatchers|BindEventtoPerformGrapplingShot _output_get (delegate Custom|Event%20GrapplingShot))
  (EventDispatchers|BindEventtoPerformRocketLaunch _asbp_top_down_controller (delegate Custom|Event%20RocketLaunch)))

(event EventTick
  (params (DeltaSeconds :type Float%20%28single-precision%29))
  (bind _grappleshootspeed (Variables|Default|GetGrappleShootSpeed))
  (bind _maxgrapplelength (Variables|Default|GetMaxGrappleLength))
  (bind _returnvalue (* DeltaSeconds _grappleshootspeed))
  (if (Variables|Default|GetIsGrappleMoving)
    (Transformation|SetActorLocation (+ (Transformation|GetActorLocation) (* (Math|Rotator|GetRotationXVector (Transformation|GetActorRotation)) (Variables|Default|GetGrappleMoveSpeed) DeltaSeconds)) false false)
    (if (<= (- (Variables|Default|GetGrappleLength) (* DeltaSeconds (/ (Variables|Default|GetGrappleMoveSpeed) 12.0))) 0.0)
      (Variables|Default|SetGrappleLength 0.0)
      (CallFunction|UpdateGrappleLength)
      (Variables|Default|SetIsGrappleMoving false)
      (Variables|/Script/Engine.CharacterMovementComponent|SetGravityScale (Variables|Character|GetCharacterMovement) 1.0)
      (Default|CallStopGrappling)
      (Rendering|SetVisibility (Variables|Default|GetGrappleHook) false false)
      (CallFunction|SetControllable true)
      (Rendering|SetVisibility (Variables|Default|GetGrappleRope) false false)
      (CallFunction|UpdateWeapon)
      (else
        (Variables|Default|SetGrappleLength (- (Variables|Default|GetGrappleLength) (* DeltaSeconds (/ (Variables|Default|GetGrappleMoveSpeed) 12.0))))
        (CallFunction|UpdateGrappleLength)))
    (elif (Variables|Default|GetIsGrappleShooting)
      (if (> (+ _returnvalue (Variables|Default|GetGrappleLength)) _maxgrapplelength)
        (Variables|Default|SetGrappleLength _maxgrapplelength)
        (CallFunction|UpdateGrappleLength)
        (Variables|Default|SetIsGrappleShooting false)
        (Variables|Default|SetIsGrappleRetracting true)
        (else
          (Variables|Default|SetGrappleLength (+ _returnvalue (Variables|Default|GetGrappleLength)))
          (CallFunction|UpdateGrappleLength)))
      (elif (Variables|Default|GetIsGrappleRetracting)
        (if (<= (- (Variables|Default|GetGrappleLength) _returnvalue) 1.0)
          (Variables|Default|SetGrappleLength 1.0)
          (CallFunction|UpdateGrappleLength)
          (Variables|Default|SetIsGrappleRetracting false)
          (Rendering|SetVisibility (Variables|Default|GetGrappleHook) false false)
          (CallFunction|SetControllable true)
          (Rendering|SetVisibility (Variables|Default|GetGrappleRope) false false)
          (Default|CallStopGrappling)
          (CallFunction|UpdateWeapon)
          (else
            (Variables|Default|SetGrappleLength (- (Variables|Default|GetGrappleLength) _returnvalue))
            (CallFunction|UpdateGrappleLength)))))))

(fn ConstructionScript
  (Variables|Default|SetInitialConeLocation (Variables|/Script/Engine.SceneComponent|GetRelativeLocation (Variables|Default|GetGrappleHook)))
  (Variables|Default|SetInitialProbeLocation (Variables|/Script/Engine.SceneComponent|GetRelativeLocation (Variables|Default|GetGrappleProbe))))

(fn UpdateWeapon
  (bind _weaponcollision (Variables|Default|GetWeaponCollision))
  (bind _weaponmesh (Variables|Default|GetWeaponMesh))
  (bind _controllerref (Variables|Default|GetControllerRef))
  (bind _weapon (Variables|/Game/TopDown/Blueprints/BP_TopDownController.BP_TopDownController_C|GetWeapon _controllerref))
  (Components|StaticMesh|SetStaticMesh _weaponmesh 0)
  (Components|Capsule|SetCapsuleHalfHeight _weaponcollision 0.0 true)
  (if (== _weapon 0)
    (Components|StaticMesh|SetStaticMesh _weaponmesh "/Game/Meshes/Stick.Stick")
    (Components|Capsule|SetCapsuleHalfHeight _weaponcollision 1.0 true)
    (Transformation|SetRelativeLocation _weaponcollision "0,0.150000,0.800000" false false)
    (Variables|Default|SetIsWeaponPiercing false)
    (Variables|Default|SetWeaponDmgDuration 0.3)
    (elif (== _weapon 1)
      (Components|StaticMesh|SetStaticMesh _weaponmesh "/Game/Meshes/Club.Club")
      (Components|Capsule|SetCapsuleHalfHeight _weaponcollision 1.0 true)
      (Transformation|SetRelativeLocation _weaponcollision "0,0.150000,0.800000" false false)
      (Variables|Default|SetIsWeaponPiercing true)
      (Variables|Default|SetWeaponDmgDuration 1.9)
      (elif (== _weapon 2)
        (Components|StaticMesh|SetStaticMesh _weaponmesh "/Game/Meshes/Sword.Sword")
        (Components|Capsule|SetCapsuleHalfHeight _weaponcollision 0.9 true)
        (Transformation|SetRelativeLocation _weaponcollision "0,0.150000,0.800000" false false)
        (Variables|Default|SetIsWeaponPiercing true)
        (Variables|Default|SetWeaponDmgDuration 0.5)))))

(fn DamageDog
  (params (Dmg :type Float%20%28double-precision%29))
  (if (Variables|Default|GetIsBlocking)
    (Animation|PlayAnimMontage "/Game/Animations/Dog/AM_BlockDog.AM_BlockDog" 1.0 "None")
    (elif (> (Variables|Default|GetHP) 0.0)
      (Audio|PlaySoundatLocation "/Game/Sounds/dog-whine_Cue.dog-whine_Cue" (Transformation|GetActorLocation) "0, 0, 0" 1.0 1.0 0.0 0 0 0 0)
      (bind _output_get (Variables|Default|SetHP (- (Variables|Default|GetHP) Dmg)))
      (if (<= _output_get 0.0)
        (Default|CallDead)
        (CallFunction|SetControllable false)))))

(fn DisplayGadget
  (bind _weaponcollision (Variables|Default|GetWeaponCollision))
  (bind _weaponmesh (Variables|Default|GetWeaponMesh))
  (bind _controllerref (Variables|Default|GetControllerRef))
  (bind _gadget (Variables|/Game/TopDown/Blueprints/BP_TopDownController.BP_TopDownController_C|GetGadget _controllerref))
  (Components|StaticMesh|SetStaticMesh _weaponmesh 0)
  (Components|Capsule|SetCapsuleHalfHeight _weaponcollision 0.0 true)
  (if (== _gadget 0)
    (Components|StaticMesh|SetStaticMesh _weaponmesh "/Game/Meshes/GrapplingGun.GrapplingGun")
    (Transformation|SetRelativeLocation _weaponcollision "0,0.150000,1.150000" false false)
    (Rendering|SetVisibility (Variables|Default|GetGrapplingHookFake) true false)
    (elif (== _gadget 1)
      (Components|StaticMesh|SetStaticMesh _weaponmesh "/Game/Meshes/GrapplingHook_Cube.GrapplingHook_Cube")
      (Transformation|SetRelativeLocation _weaponcollision "0,0.150000,1.150000" false false))))

(fn UpdateGrappleLength
  (bind _grapplerope (Variables|Default|GetGrappleRope))
  (bind _grapplelength (Variables|Default|GetGrappleLength))
  (bind _returnvalue (Transformation|GetWorldScale _grapplerope))
  (bind _returnvalue_2 (* _grapplelength 38.0))
  (bind _returnvalue_3 (Math|Vector|MakeVector 0.0 _returnvalue_2 0.0))
  (bind (_x _y) (Class|KismetMathLibrary|BreakVector3f _returnvalue))
  (Transformation|SetRelativeLocation (Variables|Default|GetGrappleProbe) (+ _returnvalue_3 (Variables|Default|GetInitialProbeLocation)) false false)
  (Transformation|SetRelativeLocation (Variables|Default|GetGrappleHook) (+ _returnvalue_3 (Variables|Default|GetInitialConeLocation)) false false)
  (Transformation|SetWorldScale3D _grapplerope (Math|Vector|MakeVector _x _y (* (Variables|Default|GetGrappleLength) (Variables|Default|GetRopeMultiplier)))))

(fn SetControllable
  (params (Controllable :type Boolean))
  (bind _output_get (Variables|Default|SetIsControllable Controllable))
  (Variables|/Game/TopDown/Blueprints/BP_TopDownController.BP_TopDownController_C|SetIsPlayerControllable (Variables|Default|GetControllerRef) _output_get))