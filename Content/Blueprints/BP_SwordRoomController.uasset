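; Sword room encounter controller that locks the player in with a wave of skeletons until they are all dead.
; When a player-tagged actor enters the trigger, it closes the door and, after a one-second delay, spawns behavior-tree skeletons at the WaveTransform points.
; While active, Tick polls the spawned list for valid references; once none remain, it reopens the door and marks the encounter completed so it cannot retrigger.
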(event OnComponentBeginOverlap(Trigger)
  (params (OverlappedComponent :type Primitive%20Component%20Object%20Reference) (OtherActor :type Actor%20Object%20Reference) (OtherComp :type Primitive%20Component%20Object%20Reference) (OtherBodyIndex :type Integer) (bFromSweep :type Boolean) (SweepResult :type Hit%20Result%20Structure%20%28by%20ref%29))
  (if (not (Variables|Default|GetBeenActivated))
    (if (not (Variables|Default|GetActivated))
      (if (Actor|ActorHasTag OtherActor "Player")
        (Default|CallCloseDoor)
        (Utilities|FlowControl|Delay 1.0)
        (CallFunction|SpawnWave)
        (Variables|Default|SetActivated true)))))

(event EventTick
  (params (DeltaSeconds :type Float%20%28single-precision%29))
  (if (Variables|Default|GetActivated)
    (Variables|Default|SetDeadFlag true)
    (bind _array_element (Utilities|Array|ForEachLoopwithBreak (Variables|Default|GetSpawnedEnemies) :!label _label)
      (:LoopBody
        (if (Utilities|IsValid _array_element)
          (Variables|Default|SetDeadFlag false)
          (goto _label Break)))
      (:Completed
        (if (Variables|Default|GetDeadFlag)
          (Default|CallOpenDoor)
          (Variables|Default|SetActivated false)
          (Variables|Default|SetBeenActivated true))))))

(fn ConstructionScript)

(fn SpawnWave
  (for _array_element (Variables|Default|GetWaveTransform)
    (bind _returnvalue (AI|SpawnAIFromClass "/Game/Blueprints/BP_Skeleton.BP_Skeleton_C" "/Game/Blueprints/BT_Skeleton.BT_Skeleton" (.location _array_element) (.rotation _array_element) false 0))
    (Utilities|Array|Add (Variables|Default|GetSpawnedEnemies) _returnvalue)))