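; BP_ColorPuzzleController runs a three-block color puzzle with two solutions, each revealing a different item.
; On BeginPlay it binds UpdateColors to each ColorBlock's change event, then checks the three ColorIndex values against two fixed combinations.
; One combination moves SkelKey to the controller's location, the other sets BonePart's height to a fixed Z.
; Both play a chime and act only while the item is valid, using relative-location setters fed with world positions.
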(event Custom|Event%20UpdateColors
  (bind _returnvalue (Transformation|GetActorLocation))
  (bind _colorblock1 (Variables|Default|GetColorBlock1))
  (bind _colorblock2 (Variables|Default|GetColorBlock2))
  (bind _skelkey (Variables|Default|GetSkelKey))
  (bind _colorblock3 (Variables|Default|GetColorBlock3))
  (bind _bonepart (Variables|Default|GetBonePart))
  (bind _returnvalue_2 (Transformation|GetActorLocation _bonepart))
  (if (Math|Boolean|ANDBoolean (== (Variables|/Game/Blueprints/BP_InteractableColorBlock.BP_InteractableColorBlock_C|GetColorIndex _colorblock1) 5) (== (Variables|/Game/Blueprints/BP_InteractableColorBlock.BP_InteractableColorBlock_C|GetColorIndex _colorblock2) 4) (== (Variables|/Game/Blueprints/BP_InteractableColorBlock.BP_InteractableColorBlock_C|GetColorIndex _colorblock3) 0))
    (Utilities|IsValid _skelkey
      (:Is%20Valid
        (Transformation|SetActorRelativeLocation _skelkey (Transformation|GetActorLocation))
        (Audio|PlaySoundatLocation "/Game/Sounds/ding-dong_Cue.ding-dong_Cue" _returnvalue "0, 0, 0" 1.0 1.0 0.0 0 0 0 0)))
    (elif (Math|Boolean|ANDBoolean (== (Variables|/Game/Blueprints/BP_InteractableColorBlock.BP_InteractableColorBlock_C|GetColorIndex _colorblock1) 1) (== (Variables|/Game/Blueprints/BP_InteractableColorBlock.BP_InteractableColorBlock_C|GetColorIndex _colorblock2) 0) (== (Variables|/Game/Blueprints/BP_InteractableColorBlock.BP_InteractableColorBlock_C|GetColorIndex _colorblock3) 3))
      (Utilities|IsValid _bonepart
        (:Is%20Valid
          (Transformation|SetActorRelativeLocation _bonepart (Math|Vector|MakeVector (.x _returnvalue_2) (.y _returnvalue_2) 42.0))
          (Audio|PlaySoundatLocation "/Game/Sounds/ding-dong_Cue.ding-dong_Cue" _returnvalue "0, 0, 0" 1.0 1.0 0.0 0 0 0 0))))))

(event EventBeginPlay
  (EventDispatchers|BindEventtoChanged (Variables|Default|GetColorBlock1) (delegate Custom|Event%20UpdateColors))
  (EventDispatchers|BindEventtoChanged (Variables|Default|GetColorBlock2) (delegate Custom|Event%20UpdateColors))
  (EventDispatchers|BindEventtoChanged (Variables|Default|GetColorBlock3) (delegate Custom|Event%20UpdateColors)))

(fn ConstructionScript)