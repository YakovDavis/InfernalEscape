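; BP_LockedFence is a fence that slides down when its referenced lock fires an unlocked event.
; On BeginPlay it binds to LockRef, and the unlock calls Open, which sets a downward direction and plays a sound.
; While moving, Tick shifts the mesh's relative Z at constant speed, clamping at TargetHeight.
; A Close function reverses the motion back to zero height but is not called within this Blueprint.
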(event Custom|Event%20Unlocked
  (CallFunction|Open))

(event EventTick
  (params (DeltaSeconds :type Float%20%28single-precision%29))
  (bind _staticmesh (Variables|Default|GetStaticMesh))
  (bind _direction (Variables|Default|GetDirection))
  (bind _direction_2 (Variables|Default|GetDirection))
  (bind _returnvalue (* DeltaSeconds _direction))
  (bind _relativelocation (Variables|/Script/Engine.SceneComponent|GetRelativeLocation _staticmesh))
  (bind _returnvalue_2 (+ (.z _relativelocation) _returnvalue))
  (if (Variables|Default|GetIsMoving)
    (if (and (< _direction_2 0.0) (< _returnvalue_2 (Variables|Default|GetTargetHeight)))
      (CallFunction|UpdateFence (Variables|Default|GetTargetHeight))
      (Variables|Default|SetIsMoving false)
      (elif (and (> _direction_2 0.0) (> _returnvalue_2 0.0))
        (CallFunction|UpdateFence 0.0)
        (Variables|Default|SetIsMoving false)
        (else
          (CallFunction|UpdateFence _returnvalue_2))))))

(event EventBeginPlay
  (EventDispatchers|BindEventtoUnlocked (Variables|Default|GetLockRef) (delegate Custom|Event%20Unlocked)))

(fn ConstructionScript)

(fn UpdateFence
  (params (Height :type Float%20%28double-precision%29))
  (bind _staticmesh (Variables|Default|GetStaticMesh))
  (bind _relativelocation (Variables|/Script/Engine.SceneComponent|GetRelativeLocation _staticmesh))
  (Transformation|SetRelativeLocation _staticmesh (Math|Vector|MakeVector (.x _relativelocation) (.y _relativelocation) Height) false false))

(fn Open
  (Variables|Default|SetIsMoving true)
  (Variables|Default|SetDirection (* (Variables|Default|GetSpeed) -1.0))
  (Audio|PlaySoundatLocation "/Game/Sounds/rise-from-sand_Cue.rise-from-sand_Cue" (Transformation|GetActorLocation) "0, 0, 0" 1.0 1.0 0.0 0 0 0 0))

(fn Close
  (Variables|Default|SetIsMoving true)
  (Variables|Default|SetDirection (* (Variables|Default|GetSpeed) 1.0))
  (Audio|PlaySoundatLocation "/Game/Sounds/rise-from-sand_Cue.rise-from-sand_Cue" (Transformation|GetActorLocation) "0, 0, 0" 1.0 1.0 0.0 0 0 0 0))