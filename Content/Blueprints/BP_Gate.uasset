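; BP_Gate is a double gate actor whose two leaves swing open and closed in mirror image around yaw.
; Open and Close set a signed speed and start movement, with Open also playing a screech sound at the gate.
; Tick advances the left leaf's yaw each frame, clamps it between closed and the open angle, then stops.
; The construction script can pose the gate open by default.
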(event EventTick
  (params (DeltaSeconds :type Float%20%28single-precision%29))
  (bind _leftpart (Variables|Default|GetLeftPart))
  (bind _direction (Variables|Default|GetDirection))
  (bind _direction_2 (Variables|Default|GetDirection))
  (bind _returnvalue (* DeltaSeconds _direction))
  (bind _relativerotation (Variables|/Script/Engine.SceneComponent|GetRelativeRotation _leftpart))
  (bind _returnvalue_2 (+ (.yaw _relativerotation) _returnvalue))
  (if (Variables|Default|GetIsMoving)
    (if (and (< _direction_2 0.0) (< _returnvalue_2 0.0))
      (CallFunction|UpdateAngle 0.0)
      (Variables|Default|SetIsMoving false)
      (elif (and (> _direction_2 0.0) (> _returnvalue_2 (Variables|Default|GetOpenAngle)))
        (CallFunction|UpdateAngle (Variables|Default|GetOpenAngle))
        (Variables|Default|SetIsMoving false)
        (else
          (CallFunction|UpdateAngle _returnvalue_2))))))

(fn ConstructionScript
  (if (Variables|Default|GetDefaultOpen)
    (CallFunction|UpdateAngle (Variables|Default|GetOpenAngle))))

(fn Open
  (Variables|Default|SetIsMoving true)
  (Variables|Default|SetDirection (* (Variables|Default|GetSpeed) 1.0))
  (Audio|PlaySoundatLocation "/Game/Sounds/gate-screech_Cue.gate-screech_Cue" (Transformation|GetActorLocation) "0, 0, 0" 1.0 1.0 0.0 0 0 0 0))

(fn UpdateAngle
  (params (Angle :type Float%20%28double-precision%29))
  (Transformation|SetRelativeRotation (Variables|Default|GetLeftPart) (Math|Rotator|MakeRotator 0.0 0.0 Angle) false false)
  (Transformation|SetRelativeRotation (Variables|Default|GetRightPart) (Math|Rotator|MakeRotator 0.0 0.0 (* Angle -1.0)) false false))

(fn Close
  (Variables|Default|SetIsMoving true)
  (Variables|Default|SetDirection (* (Variables|Default|GetSpeed) -1.0)))