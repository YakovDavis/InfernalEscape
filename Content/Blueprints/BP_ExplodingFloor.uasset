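; Floor actor that collapses when the player controller signals it to explode.
; On BeginPlay it binds its Activate event to the ExplodeFloor dispatcher on BP_TopDownController.
; Activate shows a warning decal, waits, then fires the floor's effect component and a falling-bricks sound at its location.
; After a further short delay it destroys the Plane component, leaving the actor itself in place.
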(event Custom|Event%20Activate
  (Rendering|SetVisibility (Variables|Default|GetDecal) true false)
  (Utilities|FlowControl|Delay 1.0)
  (Components|Activation|Activate (Variables|Default|GetNS_ExplodingFloor) false)
  (Audio|PlaySoundatLocation "/Game/Sounds/bricks-falling_Cue.bricks-falling_Cue" (Transformation|GetActorLocation) "0, 0, 0" 1.0 1.0 0.0 0 0 0 0)
  (Utilities|FlowControl|Delay 0.2)
  (Components|DestroyComponent (Variables|Default|GetPlane)))

(event EventBeginPlay
  (bind _asbp_top_down_controller (Utilities|Casting|CastToBP_TopDownController (Game|GetPlayerController 0)))
  (EventDispatchers|BindEventtoExplodeFloor _asbp_top_down_controller (delegate Custom|Event%20Activate)))

(event Collision|EventActorBeginOverlap
  (params (OtherActor :type Actor%20Object%20Reference)))

(event EventTick
  (params (DeltaSeconds :type Float%20%28single-precision%29)))

(fn ConstructionScript)