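; Interactable color block that advances to the next color in its list, wrapping around, whenever it is hit while active.
; On BeginPlay it creates a dynamic material instance on the cube mesh and applies the starting color.
; Normal and explosive damage handlers both cycle the index and play a sword-hit sound.
; UpdateColor sets the material's base color and fires the Changed dispatcher for any listeners, including on the initial update.
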(event EventBeginPlay
  (|CallParentFunction)
  (bind _returnvalue (Rendering|Material|CreateDynamicMaterialInstance (Variables|Default|GetCubeMesh) 0 "/Game/Materials/M_InteractiveColoredBlock.M_InteractiveColoredBlock" "None" :!class /Script/Engine.PrimitiveComponent))
  (Variables|Default|SetMatInst _returnvalue)
  (CallFunction|UpdateColor (Variables|Default|GetColorIndex)))

(fn ConstructionScript
  (|CallParentFunction))

(fn DamageEnemy
  (params (Damage :type Float%20%28double-precision%29))
  (if (Variables|Default|GetIsActive)
    (bind _output_get (Variables|Default|SetColorIndex (Math|Integer|%(Integer) (+ (Variables|Default|GetColorIndex) 1) (Utilities|Array|Length (Variables|Default|GetColorList)))))
    (CallFunction|UpdateColor _output_get)
    (Audio|PlaySoundatLocation "/Game/Sounds/sword-hit_Cue.sword-hit_Cue" (Transformation|GetActorLocation) "0, 0, 0" 1.0 1.0 0.0 0 0 0 0)))

(fn UpdateColor
  (params (Index :type Integer))
  (Rendering|Material|SetVectorParameterValue (Variables|Default|GetMatInst) "BaseColor" (Math|Conversions|ToLinearColor(Vector) (Utilities|Array|Get(acopy) (Variables|Default|GetColorList) Index)) :!class /Script/Engine.MaterialInstanceDynamic)
  (Default|CallChanged))

(fn ExplosiveDamageEnemy
  (params (Damage :type Float%20%28double-precision%29))
  (if (Variables|Default|GetIsActive)
    (bind _output_get (Variables|Default|SetColorIndex (Math|Integer|%(Integer) (+ (Variables|Default|GetColorIndex) 1) (Utilities|Array|Length (Variables|Default|GetColorList)))))
    (CallFunction|UpdateColor _output_get)
    (Audio|PlaySoundatLocation "/Game/Sounds/sword-hit_Cue.sword-hit_Cue" (Transformation|GetActorLocation) "0, 0, 0" 1.0 1.0 0.0 0 0 0 0)))