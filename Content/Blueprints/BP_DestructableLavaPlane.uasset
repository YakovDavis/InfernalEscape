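; BP_DestructableLavaPlane is a lava plane actor that dries up by sinking, then removes itself.
; On BeginPlay it binds StartDrying to a RockTrigger's HeyIveMoved event, which starts drying after a short delay.
; Tick decreases Percent over time and lowers the actor by a Percent-scaled, frame-rate-dependent step, so the descent slows.
; At zero it deactivates the linked Niagara effect, if valid, and destroys itself.
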(event Custom|Event%20StartDrying
  (Utilities|FlowControl|Delay 0.5)
  (Variables|Default|SetIsDrying true)
  (Actor|Tick|SetActorTickEnabled true))

(event EventBeginPlay
  (EventDispatchers|BindEventtoHeyIveMoved (Variables|Default|GetRockTrigger) (delegate Custom|Event%20StartDrying)))

(event EventTick
  (params (DeltaSeconds :type Float%20%28single-precision%29))
  (bind _returnvalue (Transformation|GetActorLocation))
  (bind _niagara (Variables|Default|GetNiagara))
  (if (Variables|Default|GetIsDrying)
    (if (<= (Variables|Default|GetPercent) 0.0)
      (if (Utilities|IsValid _niagara)
        (Components|Activation|Deactivate (Variables|/Script/Niagara.NiagaraActor|GetNiagaraComponent _niagara)))
      (Actor|DestroyActor)
      (else
        (bind _output_get (Variables|Default|SetPercent (- (Variables|Default|GetPercent) (* (Variables|Default|GetDryingSpeedPercent) DeltaSeconds))))
        (Transformation|SetActorLocation (Math|Vector|MakeVector (.x _returnvalue) (.y _returnvalue) (- (.z _returnvalue) (* (/ _output_get 1e+02) (Variables|Default|GetMaxOffset)))) false false)))))

(fn ConstructionScript
  (|CallParentFunction))