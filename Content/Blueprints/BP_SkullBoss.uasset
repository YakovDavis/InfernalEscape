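; BP_SkullBoss is a skull boss enemy whose fight is driven by a BossController.
; Controller signals start the battle, reset HP and active state, and trigger jaw, wand and skull animations for skeleton summons.
; While active, Tick moves the skull vertically along a repeating half sine wave.
; Damage overrides report HP back to the controller, and death plays a sound, notifies it and spawns a poof.
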(event Custom|Event%20BattleStart
  (Variables|Default|SetIsActive true))

(event Custom|Event%20SummonSkeleton
  (Components|Animation|PlayAnimation (Variables|Default|Getboss-skull_jaw) "/Game/Meshes/NewFolder/boss-skull_g_Jaw_Anim.boss-skull_g_Jaw_Anim" false)
  (Components|Animation|PlayAnimation (Variables|Default|Getboss-skull_wand) "/Game/Meshes/NewFolder/boss-skull_wand_Anim.boss-skull_wand_Anim" false)
  (Components|Animation|PlayAnimation (Variables|Default|Getboss-skull_skull) "/Game/Meshes/NewFolder/boss-skull_g_Skull_Anim.boss-skull_g_Skull_Anim" false))

(event Custom|Event%20Reset
  (Variables|Default|SetHP (Variables|Default|GetFullHP))
  (Variables|Default|SetIsActive false))

(event EventBeginPlay
  (bind _bosscontroller (Variables|Default|GetBossController))
  (|CallParentFunction)
  (if (Utilities|IsValid _bosscontroller)
    (EventDispatchers|BindEventtoBattleStartSignal _bosscontroller (delegate Custom|Event%20BattleStart))
    (EventDispatchers|BindEventtoSpawnSkeletonSignal _bosscontroller (delegate Custom|Event%20SummonSkeleton))
    (EventDispatchers|BindEventtoBattleResetSignal _bosscontroller (delegate Custom|Event%20Reset))))

(event EventTick
  (params (DeltaSeconds :type Float%20%28single-precision%29))
  (if (Variables|Default|GetIsActive)
    (bind _output_get (Variables|Default|SetWaveTime (Math|Float|%(Float) (+ (Variables|Default|GetWaveTime) DeltaSeconds) 1.8e+02)))
    (Transformation|SetRelativeLocation (Variables|Default|Getboss-skull_skull) (Math|Vector|MakeVector 0.0 0.0 (* (Math|Trig|Sin(Degrees) _output_get) 1e+02)) false false)))

(fn ConstructionScript
  (|CallParentFunction))

(fn Death
  (bind _returnvalue (Transformation|GetActorLocation))
  (Audio|PlaySoundatLocation "/Game/Sounds/skeleton_dying_Cue.skeleton_dying_Cue" _returnvalue "0, 0, 0" 1.0 1.0 0.0 0 0 0 0)
  (Default|EventBossDead (Variables|Default|GetBossController))
  (Game|SpawnActorfromClass "/Game/Blueprints/BP_Poof.BP_Poof_C" (Math|Transform|MakeTransform _returnvalue "0, 0, 0" "1.000000,1.000000,1.000000") "Undefined" 0 0)
  (|CallParentFunction))

(fn ExplosiveDamageEnemy
  (params (Damage :type Float%20%28double-precision%29))
  (|CallParentFunction Damage)
  (Default|UpdateBossHeath (Variables|Default|GetBossController) (Variables|Default|GetHP)))

(fn DamageEnemy
  (params (Damage :type Float%20%28double-precision%29))
  (|CallParentFunction Damage)
  (Default|UpdateBossHeath (Variables|Default|GetBossController) (Variables|Default|GetHP)))