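; Destructible chain linked to a drawbridge or double drawbridge that retracts upward once triggered.
; Death fires the hit call, sound and event marker once, and starts retraction unless a double drawbridge's Started event must do so.
; Tick raises and shortens the chain until minimum length or the bridge's Done event, rebuilding instanced mesh segments when their count changes.
; With a double drawbridge, losing the marker disables Death's trigger.
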(event Custom|Event%20Done
  (Variables|Default|SetIsGoingUp false)
  (Actor|Tick|SetActorTickEnabled false))

(event Custom|Event%20Started
  (if (Variables|Default|GetIsWaitingForStarted)
    (Variables|Default|SetIsGoingUp true)
    (Actor|Tick|SetActorTickEnabled true)))

(event Custom|Event%20MarkerMissing
  (Variables|Default|SetActivated true))

(event EventBeginPlay
  (bind _donedispatcher (Variables|Default|GetDoneDispatcher))
  (bind _eventmarker (Variables|Default|GetEventMarker))
  (|CallParentFunction)
  (bind _asbp_drawbridge (Utilities|Casting|CastToBP_Drawbridge _donedispatcher)
    (:then
      (EventDispatchers|BindEventtoDone _asbp_drawbridge (delegate Custom|Event%20Done)))
    (:CastFailed
      (bind _asbp_double_drawbridge (Utilities|Casting|CastToBP_DoubleDrawbridge _donedispatcher))
      (EventDispatchers|BindEventtoDone _asbp_double_drawbridge (delegate Custom|Event%20Done))
      (Variables|Default|SetIsWaitingForStarted true)
      (EventDispatchers|BindEventtoStarted _asbp_double_drawbridge (delegate Custom|Event%20Started))
      (Utilities|IsValid _eventmarker
        (:Is%20Valid
          (EventDispatchers|BindEventtoDestroyed _eventmarker (delegate Custom|Event%20MarkerMissing)))))))

(event EventTick
  (params (DeltaSeconds :type Float%20%28single-precision%29))
  (bind _speed (Variables|Default|GetSpeed))
  (bind _instancedstaticmesh (Variables|Default|GetInstancedStaticMesh))
  (bind _returnvalue (* DeltaSeconds _speed))
  (if (Variables|Default|GetIsGoingUp)
    (if (>= (Variables|Default|GetLength) (Variables|Default|GetRemainingLength))
      (Variables|Default|SetLength (- (Variables|Default|GetLength) _returnvalue))
      (Transformation|SetRelativeLocation _instancedstaticmesh (+ (Variables|/Script/Engine.SceneComponent|GetRelativeLocation _instancedstaticmesh) (Math|Vector|MakeVector 0.0 0.0 _returnvalue)) false false)
      (CallFunction|UpdateLength)
      (else
        (Variables|Default|SetIsGoingUp false)
        (Actor|Tick|SetActorTickEnabled false)))))

(fn ConstructionScript
  (|CallParentFunction)
  (CallFunction|UpdateLength))

(fn Death
  (bind _eventmarker (Variables|Default|GetEventMarker))
  (if (not (Variables|Default|GetActivated))
    (if (Variables|Default|GetIsWaitingForStarted)
      _
      (else
        (Variables|Default|SetIsGoingUp true)))
    (Default|CallHit)
    (Audio|PlaySoundatLocation "/Game/Sounds/chain-pull_Cue.chain-pull_Cue" (Transformation|GetActorLocation) "0, 0, 0" 1.0 1.0 0.0 0 0 0 0)
    (Utilities|IsValid _eventmarker
      (:Is%20Valid
        (Default|Activate _eventmarker))
      (:Is%20Not%20Valid
        _))
    (Variables|Default|SetActivated true)))

(fn UpdateLength
  (bind _length (Variables|Default|GetLength))
  (bind _segmentlength (Variables|Default|GetSegmentLength))
  (bind _returnvalue (/ _length _segmentlength))
  (bind _returnvalue_2 (Math|Float|Ceil _returnvalue))
  (if (not (== (Variables|Default|GetSegments) _returnvalue_2))
    (Components|InstancedStaticMesh|ClearInstances (Variables|Default|GetInstancedStaticMesh))
    (bind _output_get (Variables|Default|SetSegments _returnvalue_2))
    (for _index (range 0 (- _output_get 1))
      (Components|InstancedStaticMesh|AddInstance (Variables|Default|GetInstancedStaticMesh) (Math|Conversions|ToTransform(Vector) (- (* (* (Math|Vector|VectorUp) (/ (Variables|Default|GetSegmentLength) 2.0)) _index) "0,0,21.000000")) false))))