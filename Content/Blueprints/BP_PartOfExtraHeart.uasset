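; BP_PartOfExtraHeart is a collectible heart piece that the player dog picks up with the context interact input.
; Overlapping PickupRange with the player sets an in-range flag and highlights the constantly spinning Heart through custom depth.
; The Pickup event, bound through BP_TopDownController, awards the piece to BP_Dog when in range.
; It then records itself in the level save's collected pickups and destroys the actor.
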(event OnComponentBeginOverlap(PickupRange)
  (params (OverlappedComponent :type Primitive%20Component%20Object%20Reference) (OtherActor :type Actor%20Object%20Reference) (OtherComp :type Primitive%20Component%20Object%20Reference) (OtherBodyIndex :type Integer) (bFromSweep :type Boolean) (SweepResult :type Hit%20Result%20Structure%20%28by%20ref%29))
  (if (Actor|ActorHasTag OtherActor "Player")
    (Variables|Default|SetIsInRange true)
    (Rendering|SetRenderCustomDepth (Variables|Default|GetHeart) true)))

(event OnComponentEndOverlap(PickupRange)
  (params (OverlappedComponent :type Primitive%20Component%20Object%20Reference) (OtherActor :type Actor%20Object%20Reference) (OtherComp :type Primitive%20Component%20Object%20Reference) (OtherBodyIndex :type Integer))
  (if (Actor|ActorHasTag OtherActor "Player")
    (if (Utilities|Array|IsEmpty (Collision|GetOverlappingActors (Variables|Default|GetPickupRange) "/Game/Blueprints/BP_Dog.BP_Dog_C" :!class /Script/Engine.PrimitiveComponent))
      (Variables|Default|SetIsInRange false)
      (Rendering|SetRenderCustomDepth (Variables|Default|GetHeart) false))))

(event Custom|Event%20Pickup
  (if (Variables|Default|GetIsInRange)
    (Default|EventAcquirePartOfHeart (Variables|Default|GetPlayerRef))
    (bind _asbp_top_down_controller (Utilities|Casting|CastToBP_TopDownController (Game|GetPlayerController 0)))
    (Utilities|Array|AddUnique (Variables|/Game/TopDown/Blueprints/BP_LevelSaveObj.BP_LevelSaveObj_C|GetCollectedPickups (Variables|/Game/TopDown/Blueprints/BP_TopDownGameMode.BP_TopDownGameMode_C|GetLevelSaveObj (Variables|/Game/TopDown/Blueprints/BP_TopDownController.BP_TopDownController_C|GetGameModeRef _asbp_top_down_controller))) self)
    (Actor|DestroyActor)))

(event EventBeginPlay
  (bind _asbp_dog (Utilities|Casting|CastToBP_Dog (Game|Player|GetPlayerPawn 0)))
  (Variables|Default|SetPlayerRef _asbp_dog)
  (bind _asbp_top_down_controller (Utilities|Casting|CastToBP_TopDownController (Game|GetPlayerController 0)))
  (EventDispatchers|BindEventtoContextInteract _asbp_top_down_controller (delegate Custom|Event%20Pickup)))

(event EventTick
  (params (DeltaSeconds :type Float%20%28single-precision%29))
  (Transformation|AddWorldRotation (Variables|Default|GetHeart) (Math|Rotator|MakeRotator 0.0 0.0 (* DeltaSeconds (Variables|Default|GetRotationSpeed))) false false))

(fn ConstructionScript)