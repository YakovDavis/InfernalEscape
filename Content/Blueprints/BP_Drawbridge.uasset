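; Drawbridge actor that rotates to a target angle once its trigger, a destructible chain or wall, is hit.
; Tick steps the roll at constant speed, then signals done and disables itself; a marker-destroyed event snaps it straight to the target.
; Each update also re-aims an instanced-mesh chain at the Cube component, rebuilding segments only when their count changes.
; The construction script runs the same update.
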(event Custom|Event%20StartMoving
  (Variables|Default|SetIsMoving true)
  (Actor|Tick|SetActorTickEnabled true))

(event Custom|Event%20MarkerMissing
  (Variables|Default|SetAngle (Variables|Default|GetTargetAngle))
  (CallFunction|UpdateBridge)
  (Variables|Default|SetIsMoving false))

(event EventBeginPlay
  (bind _triggerobject (Variables|Default|GetTriggerObject))
  (bind _asbp_destructible_chain (Utilities|Casting|CastToBP_DestructibleChain _triggerobject)
    (:then
      (EventDispatchers|BindEventtoHit _asbp_destructible_chain (delegate Custom|Event%20StartMoving))
      (EventDispatchers|BindEventtoDestroyed (Variables|Default|GetEventMarker) (delegate Custom|Event%20MarkerMissing)))
    (:CastFailed
      (bind _asbp_destructible_wall (Utilities|Casting|CastToBP_DestructibleWall _triggerobject))
      (EventDispatchers|BindEventtoHit _asbp_destructible_wall (delegate Custom|Event%20StartMoving))
      (EventDispatchers|BindEventtoDestroyed _asbp_destructible_wall (delegate Custom|Event%20MarkerMissing)))))

(event EventTick
  (params (DeltaSeconds :type Float%20%28single-precision%29))
  (bind _movespeed (Variables|Default|GetMoveSpeed))
  (bind _returnvalue (* DeltaSeconds _movespeed))
  (if (Variables|Default|GetIsMoving)
    (if (<= (Math|Float|Absolute(Float) (- (Variables|Default|GetAngle) (Variables|Default|GetTargetAngle))) _returnvalue)
      (Variables|Default|SetAngle (Variables|Default|GetTargetAngle))
      (CallFunction|UpdateBridge)
      (Variables|Default|SetIsMoving false)
      (Default|CallDone)
      (Actor|Tick|SetActorTickEnabled false)
      (else
        (Variables|Default|SetAngle (+ (* _returnvalue (/ (- 0.0 (- (Variables|Default|GetAngle) (Variables|Default|GetTargetAngle))) (Math|Float|Absolute(Float) (- (Variables|Default|GetAngle) (Variables|Default|GetTargetAngle))))) (Variables|Default|GetAngle)))
        (CallFunction|UpdateBridge)))))

(fn ConstructionScript
  (CallFunction|UpdateBridge))

(fn UpdateBridge
  (bind _instancedstaticmesh (Variables|Default|GetInstancedStaticMesh))
  (bind _cube (Variables|Default|GetCube))
  (bind _returnvalue (Transformation|GetWorldLocation _cube))
  (bind _returnvalue_2 (Transformation|GetWorldLocation _instancedstaticmesh))
  (bind _returnvalue_3 (- _returnvalue _returnvalue_2))
  (Transformation|SetRelativeRotation (Variables|Default|GetStaticMesh) (Math|Rotator|MakeRotator (Variables|Default|GetAngle) 0.0 0.0) false false)
  (Variables|Default|SetLength (Math|Vector|VectorLength _returnvalue_3))
  (Transformation|SetWorldRotation (Variables|Default|GetInstancedStaticMesh) (Math|Conversions|RotationFromXVector (Math|Vector|CrossProduct _returnvalue_3 (Class|KismetMathLibrary|VectorLeft))) false false)
  (CallFunction|UpdateChainLength))

(fn UpdateChainLength
  (bind _length (Variables|Default|GetLength))
  (bind _segmentlength (Variables|Default|GetSegmentLength))
  (bind _returnvalue (/ _length _segmentlength))
  (bind _returnvalue_2 (Math|Float|Ceil _returnvalue))
  (if (not (== (Variables|Default|GetSegments) _returnvalue_2))
    (Components|InstancedStaticMesh|ClearInstances (Variables|Default|GetInstancedStaticMesh))
    (bind _output_get (Variables|Default|SetSegments _returnvalue_2))
    (for _index (range 0 (- _output_get 1))
      (Components|InstancedStaticMesh|AddInstance (Variables|Default|GetInstancedStaticMesh) (Math|Conversions|ToTransform(Vector) (* (* (Math|Vector|VectorUp) (/ (Variables|Default|GetSegmentLength) 2.0)) _index)) false))))