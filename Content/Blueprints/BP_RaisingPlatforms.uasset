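; Lever puzzle actor in which four two-way levers raise and lower three platforms.
; Each pull adds that lever's offset vector to unclamped virtual heights, which are clamped to a maximum to give the targets.
; Tick moves each platform toward its target at constant speed, snapping it within an error margin.
; Heights are packed as vectors, one axis per platform, in multiples of a normal height.
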(event Custom|Event%20Lever4Left
  (CallFunction|SetTargetHeights (+ (Variables|Default|GetPillarVirtualHeights) (Variables|Default|GetLever4HeightsL)))
  (Variables|Default|SetIsMoving true))

(event Custom|Event%20Lever4Right
  (CallFunction|SetTargetHeights (+ (Variables|Default|GetPillarVirtualHeights) (Variables|Default|GetLever4HeightsR)))
  (Variables|Default|SetIsMoving true))

(event Custom|Event%20Lever3Left
  (CallFunction|SetTargetHeights (+ (Variables|Default|GetPillarVirtualHeights) (Variables|Default|GetLever3HeightsL)))
  (Variables|Default|SetIsMoving true))

(event Custom|Event%20Lever3Right
  (CallFunction|SetTargetHeights (+ (Variables|Default|GetPillarVirtualHeights) (Variables|Default|GetLever3HeightsR)))
  (Variables|Default|SetIsMoving true))

(event Custom|Event%20Lever1Left
  (CallFunction|SetTargetHeights (+ (Variables|Default|GetPillarVirtualHeights) (Variables|Default|GetLever1HeightsL)))
  (Variables|Default|SetIsMoving true))

(event Custom|Event%20Lever1Right
  (CallFunction|SetTargetHeights (+ (Variables|Default|GetPillarVirtualHeights) (Variables|Default|GetLever1HeightsR)))
  (Variables|Default|SetIsMoving true))

(event Custom|Event%20Lever2Left
  (CallFunction|SetTargetHeights (+ (Variables|Default|GetPillarVirtualHeights) (Variables|Default|GetLever2HeightsL)))
  (Variables|Default|SetIsMoving true))

(event Custom|Event%20Lever2Right
  (CallFunction|SetTargetHeights (+ (Variables|Default|GetPillarVirtualHeights) (Variables|Default|GetLever2HeightsR)))
  (Variables|Default|SetIsMoving true))

(event EventBeginPlay
  (bind _lever1 (Variables|Default|GetLever1))
  (bind _lever2 (Variables|Default|GetLever2))
  (bind _lever3 (Variables|Default|GetLever3))
  (bind _lever4 (Variables|Default|GetLever4))
  (EventDispatchers|BindEventtoLeft _lever1 (delegate Custom|Event%20Lever1Left))
  (EventDispatchers|BindEventtoRight _lever1 (delegate Custom|Event%20Lever1Right))
  (EventDispatchers|BindEventtoLeft _lever2 (delegate Custom|Event%20Lever2Left))
  (EventDispatchers|BindEventtoRight _lever2 (delegate Custom|Event%20Lever2Right))
  (EventDispatchers|BindEventtoLeft _lever3 (delegate Custom|Event%20Lever3Left))
  (EventDispatchers|BindEventtoRight _lever3 (delegate Custom|Event%20Lever3Right))
  (EventDispatchers|BindEventtoLeft _lever4 (delegate Custom|Event%20Lever4Left))
  (EventDispatchers|BindEventtoRight _lever4 (delegate Custom|Event%20Lever4Right)))

(event EventTick
  (params (DeltaSeconds :type Float%20%28single-precision%29))
  (bind _err (Variables|Default|GetErr))
  (bind _targetheights (Variables|Default|GetTargetHeights))
  (if (Variables|Default|GetIsMoving)
    (bind _heights (CallFunction|GetHeights))
    (Utilities|FlowControl|Sequence
      (:then_0
        (if (and (< (Math|Float|Absolute(Float) (.x (- (Variables|Default|GetTargetHeights) (+ _heights (* (Variables|Default|GetDirections) DeltaSeconds))))) _err) (!= (.x (Variables|Default|GetDirections)) 0.0))
          (Variables|Default|SetDirections (Math|Vector|MakeVector 0.0 (.y (Variables|Default|GetDirections)) (.z (Variables|Default|GetDirections))))
          (bind _heights_2 (CallFunction|GetHeights))
          (CallFunction|SetHeights (Math|Vector|MakeVector (.x _targetheights) (.y _heights_2) (.z _heights_2)))))
      (:then_1
        (if (and (< (Math|Float|Absolute(Float) (.y (- (Variables|Default|GetTargetHeights) (+ _heights (* (Variables|Default|GetDirections) DeltaSeconds))))) _err) (!= (.y (Variables|Default|GetDirections)) 0.0))
          (Variables|Default|SetDirections (Math|Vector|MakeVector (.x (Variables|Default|GetDirections)) 0.0 (.z (Variables|Default|GetDirections))))
          (bind _heights_3 (CallFunction|GetHeights))
          (CallFunction|SetHeights (Math|Vector|MakeVector (.x _heights_3) (.y _targetheights) (.z _heights_3)))))
      (:then_2
        (if (and (< (Math|Float|Absolute(Float) (.z (- (Variables|Default|GetTargetHeights) (+ _heights (* (Variables|Default|GetDirections) DeltaSeconds))))) _err) (!= (.z (Variables|Default|GetDirections)) 0.0))
          (Variables|Default|SetDirections (Math|Vector|MakeVector (.x (Variables|Default|GetDirections)) (.y (Variables|Default|GetDirections)) 0.0))
          (bind _heights_4 (CallFunction|GetHeights))
          (CallFunction|SetHeights (Math|Vector|MakeVector (.x _heights_4) (.y _heights_4) (.z _targetheights)))))
      (:then_3
        (if (> (Math|Vector|VectorLength (Variables|Default|GetDirections)) 0.0)
          (bind _heights_5 (CallFunction|GetHeights))
          (CallFunction|SetHeights (+ _heights_5 (* (Variables|Default|GetDirections) DeltaSeconds)))
          (else
            (Variables|Default|SetIsMoving false)))))))

(fn ConstructionScript
  (CallFunction|SetHeights (Variables|Default|GetPillarVirtualHeights)))

(fn GetHeights
  (bind _normalheight (Variables|Default|GetNormalHeight))
  (return (Math|Vector|MakeVector (/ (.z (Variables|/Script/Engine.SceneComponent|GetRelativeLocation (Variables|Default|GetPlatform1))) _normalheight) (/ (.z (Variables|/Script/Engine.SceneComponent|GetRelativeLocation (Variables|Default|GetPlatform2))) _normalheight) (/ (.z (Variables|/Script/Engine.SceneComponent|GetRelativeLocation (Variables|Default|GetPlatform3))) _normalheight))))

(fn SetHeights
  (params (Heights :type Vector))
  (bind _platform1 (Variables|Default|GetPlatform1))
  (bind _platform2 (Variables|Default|GetPlatform2))
  (bind _platform3 (Variables|Default|GetPlatform3))
  (bind _normalheight (Variables|Default|GetNormalHeight))
  (bind _relativelocation (Variables|/Script/Engine.SceneComponent|GetRelativeLocation _platform3))
  (bind _relativelocation_2 (Variables|/Script/Engine.SceneComponent|GetRelativeLocation _platform1))
  (bind _relativelocation_3 (Variables|/Script/Engine.SceneComponent|GetRelativeLocation _platform2))
  (Transformation|SetRelativeLocation _platform1 (Math|Vector|MakeVector (.x _relativelocation_2) (.y _relativelocation_2) (* (.x Heights) _normalheight)) false false)
  (Transformation|SetRelativeLocation _platform2 (Math|Vector|MakeVector (.x _relativelocation_3) (.y _relativelocation_3) (* (.y Heights) _normalheight)) false false)
  (Transformation|SetRelativeLocation _platform3 (Math|Vector|MakeVector (.x _relativelocation) (.y _relativelocation) (* (.z Heights) _normalheight)) false false))

(fn SetTargetHeights
  (params (Heights :type Vector))
  (bind _maxheight (Variables|Default|GetMaxHeight))
  (bind _speed (Variables|Default|GetSpeed))
  (bind _returnvalue (* _speed 1.0))
  (bind _returnvalue_2 (* _speed -1.0))
  (Variables|Default|SetPillarVirtualHeights (Math|Vector|MakeVector (.x Heights) (.y Heights) (.z Heights)))
  (bind _output_get (Variables|Default|SetTargetHeights (Math|Vector|MakeVector (Math|Float|Clamp(Float) (.x Heights) 0.0 _maxheight) (Math|Float|Clamp(Float) (.y Heights) 0.0 _maxheight) (Math|Float|Clamp(Float) (.z Heights) 0.0 _maxheight))))
  (bind _heights (CallFunction|GetHeights))
  (Utilities|FlowControl|Sequence
    (:then_0
      (if (> (.x (- _heights _output_get)) 0.0)
        (Variables|Default|SetDirections (Math|Vector|MakeVector _returnvalue_2 (.y (Variables|Default|GetDirections)) (.z (Variables|Default|GetDirections))))
        (elif (== (.x (- _heights _output_get)) 0.0)
          (Variables|Default|SetDirections (Math|Vector|MakeVector 0.0 (.y (Variables|Default|GetDirections)) (.z (Variables|Default|GetDirections))))
          (else
            (Variables|Default|SetDirections (Math|Vector|MakeVector _returnvalue (.y (Variables|Default|GetDirections)) (.z (Variables|Default|GetDirections))))))))
    (:then_1
      (if (> (.y (- _heights _output_get)) 0.0)
        (Variables|Default|SetDirections (Math|Vector|MakeVector (.x (Variables|Default|GetDirections)) _returnvalue_2 (.z (Variables|Default|GetDirections))))
        (elif (== (.y (- _heights _output_get)) 0.0)
          (Variables|Default|SetDirections (Math|Vector|MakeVector (.x (Variables|Default|GetDirections)) 0.0 (.z (Variables|Default|GetDirections))))
          (else
            (Variables|Default|SetDirections (Math|Vector|MakeVector (.x (Variables|Default|GetDirections)) _returnvalue (.z (Variables|Default|GetDirections))))))))
    (:then_2
      (if (> (.z (- _heights _output_get)) 0.0)
        (Variables|Default|SetDirections (Math|Vector|MakeVector (.x (Variables|Default|GetDirections)) (.y (Variables|Default|GetDirections)) _returnvalue_2))
        (elif (== (.z (- _heights _output_get)) 0.0)
          (Variables|Default|SetDirections (Math|Vector|MakeVector (.x (Variables|Default|GetDirections)) (.y (Variables|Default|GetDirections)) 0.0))
          (else
            (Variables|Default|SetDirections (Math|Vector|MakeVector (.x (Variables|Default|GetDirections)) (.y (Variables|Default|GetDirections)) _returnvalue))))))))