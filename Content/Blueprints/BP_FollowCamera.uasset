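; BP_FollowCamera is a camera rig that follows the player's BP_Dog pawn.
; On BeginPlay it casts the player pawn to BP_Dog and caches the reference.
; Each tick it moves its spring arm to the dog's location and applies an offset as the arm's target offset.
; When IsLocked is set, it holds the spring arm at LockLocation instead, leaving the target offset unchanged.
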(event EventBeginPlay
  (bind _asbp_dog (Utilities|Casting|CastToBP_Dog (Game|Player|GetPlayerPawn 0)))
  (Variables|Default|SetPlayerRef _asbp_dog))

(event EventTick
  (params (DeltaSeconds :type Float%20%28single-precision%29))
  (bind _springarm (Variables|Default|GetSpringArm))
  (if (Variables|Default|GetIsLocked)
    (Transformation|SetWorldLocation _springarm (Variables|Default|GetLockLocation) false false)
    (else
      (Transformation|SetWorldLocation _springarm (Transformation|GetActorLocation (Variables|Default|GetPlayerRef)) false false)
      (Variables|/Script/Engine.SpringArmComponent|SetTargetOffset (Variables|Default|GetSpringArm) (Variables|Default|GetOffset)))))

(fn ConstructionScript)