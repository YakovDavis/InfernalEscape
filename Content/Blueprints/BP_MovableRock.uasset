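; A pushable puzzle rock that slides a fixed distance when the player keeps pressing against a side, then falls if unsupported.
; Hit normals pick one of four allowed directions, and a move timer starts if that side's probe is clear, with continued hits refreshing a cancel timer.
; Tick steps the rock to its target, calls HeyIveMoved, and repeats drops while the fall probe overlaps no static meshes, ignoring lava planes.
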(event OnComponentHit(Cube)
  (params (HitComponent :type Primitive%20Component%20Object%20Reference) (OtherActor :type Actor%20Object%20Reference) (OtherComp :type Primitive%20Component%20Object%20Reference) (NormalImpulse :type Vector :default "0, 0, 0") (Hit :type Hit%20Result%20Structure%20%28by%20ref%29))
  (bind _normal (Collision|BreakHitResult Hit))
  (bind (_x _y) (Math|Vector|BreakVector _normal))
  (if (not (or (Variables|Default|GetIsMoving) (Variables|Default|GetIsFalling)))
    (if (Utilities|Time|IsTimerActivebyHandle (Variables|Default|GetTimerToMove))
      (bind _returnvalue (Utilities|Time|SetTimerbyEvent (delegate Custom|Event%20CancelMove) (Variables|Default|GetTimeToCancel)))
      (Variables|Default|SetTimerToCancel _returnvalue)
      (elif (Variables|Default|GetCanMoveNow)
        (if (Actor|ActorHasTag OtherActor "Player")
          (if (and (Variables|Default|GetCanMoveUp) (> _x 0.1))
            (bind _result (CallFunction|GetIsNotOverlappingSMs (Variables|Default|GetProbePX)))
            (if _result
              (Variables|Default|SetMoveVector (Class|KismetMathLibrary|VectorForward))
              (bind _returnvalue_2 (Utilities|Time|SetTimerbyEvent (delegate Custom|Event%20Move) (Variables|Default|GetTimeToMove) :!label _label))
              (Variables|Default|SetTimerToMove _returnvalue_2)
              (Variables|Default|SetTargetLocation (+ (Transformation|GetActorLocation) (* (Variables|Default|GetMoveVector) (Variables|Default|GetMoveDistance))))
              (bind _returnvalue_3 (Utilities|Time|SetTimerbyEvent (delegate Custom|Event%20CancelMove) (Variables|Default|GetTimeToCancel)))
              (Variables|Default|SetTimerToCancel _returnvalue_3))
            (elif (and (Variables|Default|GetCanMoveDown) (< _x -0.1))
              (bind _result_2 (CallFunction|GetIsNotOverlappingSMs (Variables|Default|GetProbeNX)))
              (if _result_2
                (Variables|Default|SetMoveVector (Class|KismetMathLibrary|VectorBackward))
                (goto _label))
              (elif (and (> _y 0.1) (Variables|Default|GetCanMoveRight))
                (bind _result_3 (CallFunction|GetIsNotOverlappingSMs (Variables|Default|GetProbePY)))
                (if _result_3
                  (Variables|Default|SetMoveVector (Class|KismetMathLibrary|VectorRight))
                  (goto _label))
                (elif (and (Variables|Default|GetCanMoveLeft) (< _y -0.1))
                  (bind _result_4 (CallFunction|GetIsNotOverlappingSMs (Variables|Default|GetProbeNY)))
                  (if _result_4
                    (Variables|Default|SetMoveVector (Class|KismetMathLibrary|VectorLeft))
                    (goto _label)))))))))))

(event Custom|Event%20Move
  (Variables|Default|SetIsMoving true)
  (Audio|PlaySoundatLocation "/Game/Sounds/rock_moving_Cue.rock_moving_Cue" (Transformation|GetActorLocation) "0, 0, 0" 1.0 1.0 0.0 0 0 0 0))

(event Custom|Event%20CancelMove
  (Utilities|Time|ClearandInvalidateTimerbyHandle (Variables|Default|GetTimerToMove)))

(event EventTick
  (params (DeltaSeconds :type Float%20%28single-precision%29))
  (bind _returnvalue (Transformation|GetActorLocation))
  (bind _returnvalue_2 (Math|Vector|VectorDown))
  (bind _movespeed (Variables|Default|GetMoveSpeed))
  (bind _movevector (Variables|Default|GetMoveVector))
  (bind _fallspeed (Variables|Default|GetFallSpeed))
  (bind _returnvalue_3 (* DeltaSeconds _fallspeed))
  (bind _returnvalue_4 (* DeltaSeconds _movespeed))
  (bind _returnvalue_5 (* _returnvalue_4 _movevector))
  (bind _returnvalue_6 (* _returnvalue_3 _returnvalue_2))
  (bind _returnvalue_7 (+ _returnvalue_5 _returnvalue))
  (bind _returnvalue_8 (+ _returnvalue_6 _returnvalue))
  (if (Variables|Default|GetIsMoving)
    (if (> (Math|Vector|VectorLength (- _returnvalue_7 (Variables|Default|GetTargetLocation))) (Math|Vector|VectorLength _returnvalue_5))
      (Transformation|SetActorLocation _returnvalue_7 false false)
      (else
        (Transformation|SetActorLocation (Variables|Default|GetTargetLocation) false false)
        (Variables|Default|SetIsMoving false)
        (Default|CallHeyIveMoved)
        (bind _result (CallFunction|GetIsNotOverlappingSMs (Variables|Default|GetProbeFall) :!label _label))
        (if _result
          (Variables|Default|SetIsFalling true)
          (Variables|Default|SetTargetLocation (+ (Variables|Default|GetTargetLocation) (* (Variables|Default|GetFallDistance) (Math|Vector|VectorDown)))))))
    (elif (Variables|Default|GetIsFalling)
      (if (> (Math|Vector|VectorLength (- _returnvalue_8 (Variables|Default|GetTargetLocation))) (Math|Vector|VectorLength _returnvalue_6))
        (Transformation|SetActorLocation _returnvalue_8 false false)
        (else
          (Transformation|SetActorLocation (Variables|Default|GetTargetLocation) false false)
          (Variables|Default|SetIsFalling false)
          (Default|CallHeyIveMoved)
          (goto _label))))))

(fn ConstructionScript)

(fn GetIsNotOverlappingSMs
  (params (Collider :type Sphere%20Component%20Object%20Reference))
  (LocalVariables|SetResTmp false)
  (bind _array_element (Utilities|Array|ForEachLoopwithBreak (Class|PrimitiveComponent|GetOverlappingComponents Collider) :!label _label)
    (:LoopBody
      (Utilities|Casting|CastToStaticMeshComponent _array_element)
      (Utilities|Casting|CastToBP_LavaPlane (Components|GetOwner _array_element)
        (:CastFailed
          (LocalVariables|SetResTmp true)
          (goto _label Break))))
    (:Completed
      (return (not (LocalVariables|GetResTmp))))))