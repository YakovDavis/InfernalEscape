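; BP_DestructibleWall is a wall that breaks when hit by explosive damage.
; The construction script sizes two crack components and the Niagara explosion's spawn box from the actor's scale.
; On damage it calls Hit, removes the cube, plays the explosion effect and falling-brick sound, then destroys itself after a short timer.
; Before destruction it records itself in the level save's CollectedPickups list, and on Destroyed it calls Destroyed.
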(event EventBeginPlay)

(event Collision|EventActorBeginOverlap
  (params (OtherActor :type Actor%20Object%20Reference)))

(event EventTick
  (params (DeltaSeconds :type Float%20%28single-precision%29)))

(event EventDestroyed
  (Default|CallDestroyed))

(fn ConstructionScript
  (bind _returnvalue (Transformation|GetActorScale3D))
  (bind _returnvalue_2 (* (.z _returnvalue) 0.19))
  (Transformation|SetWorldScale3D (Variables|Default|GetCrack1) (Math|Vector|MakeVector _returnvalue_2 _returnvalue_2 _returnvalue_2))
  (Transformation|SetWorldScale3D (Variables|Default|GetCrack2) (Math|Vector|MakeVector _returnvalue_2 _returnvalue_2 _returnvalue_2))
  (Effects|Components|ParticleSystem|SetVectorParameter (Variables|Default|GetNS_DestructableWallExplosion) "SpawnBoxDimensions" (/ (* (Transformation|GetActorScale3D) "100.000000,100.000000,100.000000") "2.000000,2.000000,2.000000")))

(fn ExplosiveDamageEnemy
  (params (Damage :type Float%20%28double-precision%29))
  (Default|CallHit)
  (Components|DestroyComponent (Variables|Default|GetCube))
  (Components|Activation|Activate (Variables|Default|GetNS_DestructableWallExplosion) false)
  (Utilities|Time|SetTimerbyFunctionName 0 "DestroySelf" 3.0)
  (Audio|PlaySoundatLocation "/Game/Sounds/bricks-falling_Cue.bricks-falling_Cue" (Transformation|GetActorLocation) "0, 0, 0" 1.0 1.0 0.0 0 0 0 0))

(fn DestroySelf
  (bind _asbp_top_down_controller (Utilities|Casting|CastToBP_TopDownController (Game|GetPlayerController 0)))
  (Utilities|Array|AddUnique (Variables|/Game/TopDown/Blueprints/BP_LevelSaveObj.BP_LevelSaveObj_C|GetCollectedPickups (Variables|/Game/TopDown/Blueprints/BP_TopDownGameMode.BP_TopDownGameMode_C|GetLevelSaveObj (Variables|/Game/TopDown/Blueprints/BP_TopDownController.BP_TopDownController_C|GetGameModeRef _asbp_top_down_controller))) self)
  (Actor|DestroyActor))