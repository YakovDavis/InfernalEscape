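; Padlock actor that the player opens with the matching key, identified by KeyIndex.
; While the player is in the trigger, it outlines its meshes via custom depth and has BP_TopDownController show the required key, blacked out if missing.
; The controller's interact event starts a timed sequence: tilt, then poof effect, Unlocked broadcast and self-destruction.
; Unlocking also records the lock in the level save's CollectedPickups.
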(event OnComponentBeginOverlap(TriggerRange)
  (params (OverlappedComponent :type Primitive%20Component%20Object%20Reference) (OtherActor :type Actor%20Object%20Reference) (OtherComp :type Primitive%20Component%20Object%20Reference) (OtherBodyIndex :type Integer) (bFromSweep :type Boolean) (SweepResult :type Hit%20Result%20Structure%20%28by%20ref%29))
  (bind _keyindex (Variables|Default|GetKeyIndex))
  (if (Actor|ActorHasTag OtherActor "Player")
    (Variables|Default|SetInRange true)
    (Rendering|SetRenderCustomDepth (Variables|Default|GetBody) true)
    (Rendering|SetRenderCustomDepth (Variables|Default|GetArc) true)
    (Rendering|SetRenderCustomDepth (Variables|Default|GetCylinder) true)
    (Default|RequireItem (Variables|Default|GetControllerRef) _keyindex (not (Utilities|Array|Get(acopy) (Variables|/Game/TopDown/Blueprints/BP_TopDownController.BP_TopDownController_C|GetKeys (Variables|Default|GetControllerRef)) _keyindex)))))

(event OnComponentEndOverlap(TriggerRange)
  (params (OverlappedComponent :type Primitive%20Component%20Object%20Reference) (OtherActor :type Actor%20Object%20Reference) (OtherComp :type Primitive%20Component%20Object%20Reference) (OtherBodyIndex :type Integer))
  (if (Actor|ActorHasTag OtherActor "Player")
    (if (Utilities|Array|IsEmpty (Collision|GetOverlappingActors (Variables|Default|GetTriggerRange) "/Game/Blueprints/BP_Dog.BP_Dog_C" :!class /Script/Engine.PrimitiveComponent))
      (Variables|Default|SetInRange false)
      (Rendering|SetRenderCustomDepth (Variables|Default|GetBody) false)
      (Rendering|SetRenderCustomDepth (Variables|Default|GetArc) false)
      (Rendering|SetRenderCustomDepth (Variables|Default|GetCylinder) false)
      (Default|StopRequireItem (Variables|Default|GetControllerRef)))))

(event Custom|Event%20TryOpen
  (if (Variables|Default|GetInRange)
    (if (Utilities|Array|Get(acopy) (Variables|/Game/TopDown/Blueprints/BP_TopDownController.BP_TopDownController_C|GetKeys (Variables|Default|GetControllerRef)) (Variables|Default|GetKeyIndex))
      (CallFunction|StartUnlockSequence))))

(event EventBeginPlay
  (bind _asbp_top_down_controller (Utilities|Casting|CastToBP_TopDownController (Game|GetPlayerController 0)))
  (bind _output_get (Variables|Default|SetControllerRef _asbp_top_down_controller))
  (EventDispatchers|BindEventtoContextInteract _output_get (delegate Custom|Event%20TryOpen)))

(event EventDestroyed
  (Default|CallDestroyed))

(fn ConstructionScript)

(fn StartUnlockSequence
  (Audio|PlaySoundatLocation "/Game/Sounds/key-opens-lock_Cue.key-opens-lock_Cue" (Transformation|GetActorLocation) "0, 0, 0" 1.0 1.0 0.0 0 0 0 0)
  (Transformation|SetRelativeRotation (Variables|Default|GetCylinder) "0.000000, 0,-15.000000" false false)
  (Transformation|SetRelativeRotation (Variables|Default|GetBody) "0.000000, 0,-15.000000" false false)
  (Utilities|Time|SetTimerbyFunctionName 0 "FinishUnlockSequence" 1.0))

(fn FinishUnlockSequence
  (Default|CallUnlocked)
  (Components|Activation|Activate (Variables|Default|GetNS_Poof) false)
  (Rendering|SetVisibility (Variables|Default|GetBody) false false)
  (Rendering|SetVisibility (Variables|Default|GetCylinder) false false)
  (Rendering|SetVisibility (Variables|Default|GetArc) false false)
  (Utilities|Time|SetTimerbyFunctionName 0 "DestroySelf" 1.0)
  (Utilities|Array|AddUnique (Variables|/Game/TopDown/Blueprints/BP_LevelSaveObj.BP_LevelSaveObj_C|GetCollectedPickups (Variables|/Game/TopDown/Blueprints/BP_TopDownGameMode.BP_TopDownGameMode_C|GetLevelSaveObj (Variables|/Game/TopDown/Blueprints/BP_TopDownController.BP_TopDownController_C|GetGameModeRef (Variables|Default|GetControllerRef)))) self)
  (Audio|PlaySoundatLocation "/Game/Sounds/poof_Cue.poof_Cue" (Transformation|GetActorLocation) "0, 0, 0" 1.0 1.0 0.0 0 0 0 0))

(fn DestroySelf
  (Actor|DestroyActor))