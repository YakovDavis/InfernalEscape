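; BP_SpawnPoint is a checkpoint that sets the player's respawn location and saves progress.
; When a Player-tagged actor enters ActivationRange, it writes its transform, raised by ZOffset, to BP_TopDownController, then saves level data through the game mode and player data through the controller.
; Only the first overlap activates the Niagara effect and, if IsTutorial is set, shows a controls hint through the controller.
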(event OnComponentBeginOverlap(ActivationRange)
  (params (OverlappedComponent :type Primitive%20Component%20Object%20Reference) (OtherActor :type Actor%20Object%20Reference) (OtherComp :type Primitive%20Component%20Object%20Reference) (OtherBodyIndex :type Integer) (bFromSweep :type Boolean) (SweepResult :type Hit%20Result%20Structure%20%28by%20ref%29))
  (bind _returnvalue (Transformation|GetActorTransform))
  (if (Actor|ActorHasTag OtherActor "Player")
    (bind _asbp_top_down_controller (Utilities|Casting|CastToBP_TopDownController (Game|GetPlayerController 0)))
    (Variables|/Game/TopDown/Blueprints/BP_TopDownController.BP_TopDownController_C|SetRespawnLocation _asbp_top_down_controller (Math|Transform|MakeTransform (+ (.location _returnvalue) (Math|Vector|MakeVector 0.0 0.0 (Variables|Default|GetZOffset))) (.rotation _returnvalue) "1.000000,1.000000,1.000000"))
    (Default|SaveLevelData (Variables|/Game/TopDown/Blueprints/BP_TopDownController.BP_TopDownController_C|GetGameModeRef _asbp_top_down_controller))
    (Default|SavePlayerData _asbp_top_down_controller)
    (if (not (Variables|Default|GetIsActivated))
      (Components|Activation|Activate (Variables|Default|GetNiagara) false)
      (Variables|Default|SetIsActivated true)
      (if (Variables|Default|GetIsTutorial)
        (bind _asbp_top_down_controller_2 (Utilities|Casting|CastToBP_TopDownController (Game|GetPlayerController 0)))
        (Variables|/Game/TopDown/Blueprints/BP_TopDownController.BP_TopDownController_C|SetHintText _asbp_top_down_controller_2 "WASD or Left Thumbstick to move 
E or Bottom Face Button to interact 
Esc or Start Button to pause")
        (Default|CallShowHint _asbp_top_down_controller_2)))))

(fn ConstructionScript)