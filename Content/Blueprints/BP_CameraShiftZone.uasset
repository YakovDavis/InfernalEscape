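; A camera shift zone that offsets the referenced camera while a Player-tagged actor is inside its box.
; Each tick it scales TargetOffset by clamped linear X and Y falloffs from the zone's origin, multiplied together, so the shift peaks at the center.
; Overlap events toggle ticking, and on exit the offset resets to zero only once no BP_Dog remains in the box.
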(event OnComponentBeginOverlap(Box)
  (params (OverlappedComponent :type Primitive%20Component%20Object%20Reference) (OtherActor :type Actor%20Object%20Reference) (OtherComp :type Primitive%20Component%20Object%20Reference) (OtherBodyIndex :type Integer) (bFromSweep :type Boolean) (SweepResult :type Hit%20Result%20Structure%20%28by%20ref%29))
  (if (Actor|ActorHasTag OtherActor "Player")
    (Variables|Default|SetInsideBounds true)
    (Actor|Tick|SetActorTickEnabled true)))

(event OnComponentEndOverlap(Box)
  (params (OverlappedComponent :type Primitive%20Component%20Object%20Reference) (OtherActor :type Actor%20Object%20Reference) (OtherComp :type Primitive%20Component%20Object%20Reference) (OtherBodyIndex :type Integer))
  (if (Actor|ActorHasTag OtherActor "Player")
    (if (Utilities|Array|IsEmpty (Collision|GetOverlappingActors (Variables|Default|GetBox) "/Game/Blueprints/BP_Dog.BP_Dog_C" :!class /Script/Engine.PrimitiveComponent))
      (Variables|Default|SetInsideBounds false)
      (Actor|Tick|SetActorTickEnabled false)
      (Variables|/Game/Blueprints/BP_FollowCamera.BP_FollowCamera_C|SetOffset (Variables|Default|GetCameraRef) "0, 0, 0"))))

(event EventTick
  (params (DeltaSeconds :type Float%20%28single-precision%29))
  (bind _returnvalue (Transformation|GetActorLocation))
  (bind _returnvalue_2 (Game|Player|GetPlayerPawn 0))
  (bind (_x _y) (Class|KismetMathLibrary|BreakVector3f _returnvalue))
  (bind _returnvalue_3 (Transformation|GetActorLocation _returnvalue_2))
  (bind (_x_2 _y_2) (Class|KismetMathLibrary|BreakVector3f _returnvalue_3))
  (if (Variables|Default|GetInsideBounds)
    (Variables|/Game/Blueprints/BP_FollowCamera.BP_FollowCamera_C|SetOffset (Variables|Default|GetCameraRef) (* (Variables|Default|GetTargetOffset) (* (Math|Float|Clamp(Float) (- 1.0 (/ (Math|Float|Absolute(Float) (- _x_2 _x)) (Variables|Default|GetEffectStartX)))) (Math|Float|Clamp(Float) (- 1.0 (/ (Math|Float|Absolute(Float) (- _y_2 _y)) (Variables|Default|GetEffectStartY)))))))))

(fn ConstructionScript)