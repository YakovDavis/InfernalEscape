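; BP_BossController runs the boss encounter: a living player entering its box starts the fight, swapping music, showing boss HP and locking the follow camera.
; Alternating timers signal and then spawn skeletons up to a cap, while Tick prunes invalid ones.
; Player death resets the fight and clears skeletons.
; Boss death triggers the win sequence, or spawns a new skull boss if the player is dead.
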(event OnComponentBeginOverlap(Box)
  (params (OverlappedComponent :type Primitive%20Component%20Object%20Reference) (OtherActor :type Actor%20Object%20Reference) (OtherComp :type Primitive%20Component%20Object%20Reference) (OtherBodyIndex :type Integer) (bFromSweep :type Boolean) (SweepResult :type Hit%20Result%20Structure%20%28by%20ref%29))
  (bind _followcamera (Variables|Default|GetFollowCamera))
  (if (not (Variables|Default|GetIsWon))
    (if (not (Variables|Default|GetIsActive))
      (if (Actor|ActorHasTag OtherActor "Player")
        (bind _asbp_dog (Utilities|Casting|CastToBP_Dog OtherActor))
        (if (> (Variables|/Game/Blueprints/BP_Dog.BP_Dog_C|GetHP _asbp_dog) 0.0)
          (Actor|Tick|SetActorTickEnabled true)
          (Variables|Default|SetIsActive true)
          (Default|CallBattleStartSignal)
          (CallFunction|PreSpawnSkeleton)
          (bind _asbp_top_down_controller (Utilities|Casting|CastToBP_TopDownController (Game|GetPlayerController 0)))
          (Default|PauseMusic _asbp_top_down_controller)
          (bind _returnvalue (Audio|SpawnSoundatLocation "/Game/Sounds/boss_Cue.boss_Cue" "1180.000000,2760.000000,40.000000" "0, 0, 0" 1.0 1.0 0.0 0 0))
          (Variables|Default|SetBossMusic _returnvalue)
          (Default|CallShowBossHP (Variables|Default|GetControllerRef))
          (Variables|/Game/Blueprints/BP_FollowCamera.BP_FollowCamera_C|SetLockLocation _followcamera "900.000000,3100.000000,300.000000")
          (Variables|/Game/Blueprints/BP_FollowCamera.BP_FollowCamera_C|SetIsLocked _followcamera true))))))

(event Custom|Event%20PlayerDead
  (bind _bossmusic (Variables|Default|GetBossMusic))
  (bind _spawnedskeletons (Variables|Default|GetSpawnedSkeletons))
  (Variables|/Game/Blueprints/BP_FollowCamera.BP_FollowCamera_C|SetIsLocked (Variables|Default|GetFollowCamera) false)
  (if (Variables|Default|GetIsActive)
    (Default|CallHideBossHP (Variables|Default|GetControllerRef))
    (Default|CallBattleResetSignal)
    (Variables|Default|SetIsActive false)
    (for _array_element _spawnedskeletons
      (Actor|DestroyActor _array_element))
    (Utilities|Array|Clear _spawnedskeletons)
    (bind _asbp_top_down_controller (Utilities|Casting|CastToBP_TopDownController (Game|GetPlayerController 0)))
    (Default|UnpauseMusic _asbp_top_down_controller)
    (Utilities|IsValid _bossmusic
      (:Is%20Valid
        (Audio|Components|Audio|Stop _bossmusic)))))

(event Custom|Event%20BossDead
  (if (> (Variables|/Game/Blueprints/BP_Dog.BP_Dog_C|GetHP (Variables|Default|GetPlayerRef)) 0.0)
    (CallFunction|WinSequence)
    (else
      (Game|SpawnActorfromClass "/Game/Blueprints/BP_SkullBoss.BP_SkullBoss_C" (Math|Transform|MakeTransform "1150.000000,3790.000000,258.000000" "0, 0, 0" "1.000000,1.000000,1.000000") "Undefined" 0 0))))

(event EventTick
  (params (DeltaSeconds :type Float%20%28single-precision%29))
  (for (_array_element _array_index) (Variables|Default|GetSpawnedSkeletons)
    (if (not (Utilities|IsValid _array_element))
      (Utilities|Array|RemoveIndex (Variables|Default|GetSpawnedSkeletons) _array_index))))

(event EventBeginPlay
  (bind _asbp_dog (Utilities|Casting|CastToBP_Dog (Game|Player|GetPlayerPawn 0)))
  (bind _output_get (Variables|Default|SetPlayerRef _asbp_dog))
  (EventDispatchers|BindEventtoDead _output_get (delegate Custom|Event%20PlayerDead))
  (bind _asbp_top_down_controller (Utilities|Casting|CastToBP_TopDownController (Game|GetPlayerController 0)))
  (Variables|Default|SetControllerRef _asbp_top_down_controller))

(fn ConstructionScript)

(fn SpawnSkeleton
  (bind _returnvalue (Transformation|GetActorTransform))
  (if (Variables|Default|GetIsActive)
    (bind _returnvalue_2 (AI|SpawnAIFromClass "/Game/Blueprints/BP_Skeleton.BP_Skeleton_C" "/Game/Blueprints/BT_Skeleton.BT_Skeleton" (.location _returnvalue) (.rotation _returnvalue) false 0))
    (bind _asbp_skeleton (Utilities|Casting|CastToBP_Skeleton _returnvalue_2))
    (Utilities|Array|Add (Variables|Default|GetSpawnedSkeletons) _asbp_skeleton)
    (Utilities|Time|SetTimerbyFunctionName 0 "PreSpawnSkeleton" (- (Variables|Default|GetSpawnInterval) (Variables|Default|GetAnimLength)))
    (Game|SpawnActorfromClass "/Game/Blueprints/BP_Poof.BP_Poof_C" (Transformation|GetActorTransform _asbp_skeleton) "Undefined" 0 0)))

(fn PreSpawnSkeleton
  (if (< (Utilities|Array|Length (Variables|Default|GetSpawnedSkeletons)) (Variables|Default|GetMaxSkeletons))
    (Default|CallSpawnSkeletonSignal)
    (Utilities|Time|SetTimerbyFunctionName 0 "SpawnSkeleton" (Variables|Default|GetAnimLength))
    (else
      (Utilities|Time|SetTimerbyFunctionName 0 "PreSpawnSkeleton" (Variables|Default|GetSpawnInterval)))))

(fn WinSequence
  (Variables|Default|SetIsWon true)
  (Default|CallWon (Variables|Default|GetPlayerRef))
  (for _array_element (Variables|Default|GetSpawnedSkeletons)
    (Default|MakePoof _array_element)
    (Actor|DestroyActor _array_element))
  (Default|CallBattleResetSignal)
  (bind _asbp_top_down_controller (Utilities|Casting|CastToBP_TopDownController (Game|GetPlayerController 0)))
  (Variables|/Game/TopDown/Blueprints/BP_TopDownController.BP_TopDownController_C|SetIsPlayerControllable _asbp_top_down_controller false)
  (Variables|Default|SetIsActive false)
  (Audio|Components|Audio|Stop (Variables|Default|GetBossMusic))
  (Variables|/Game/Blueprints/BP_Dog.BP_Dog_C|SetHP (Variables|Default|GetPlayerRef) 1e+02)
  (Default|CallHideBossHP (Variables|Default|GetControllerRef))
  (Audio|PlaySoundatLocation "/Game/Sounds/ding-dong_Cue.ding-dong_Cue" (Transformation|GetActorLocation) "0, 0, 0" 1.0 1.0 0.0 0 0 0 0))

(fn UpdateBossHeath
  (params (HP :type Float%20%28double-precision%29))
  (bind _asbp_top_down_controller (Utilities|Casting|CastToBP_TopDownController (Game|GetPlayerController 0)))
  (Variables|/Game/TopDown/Blueprints/BP_TopDownController.BP_TopDownController_C|SetBossHealth _asbp_top_down_controller HP))