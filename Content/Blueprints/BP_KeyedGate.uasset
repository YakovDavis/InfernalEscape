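; BP_KeyedGate is a gate that opens in response to a referenced lock.
; On BeginPlay it runs the parent logic, then binds to the lock's Unlocked and Destroyed events.
; Unlocking calls Open, while destruction of the lock passes OpenAngle straight to UpdateAngle.
; The gate movement functions are not defined here, and Tick and overlap events are disabled stubs.
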(event Custom|Event%20Open
  (CallFunction|Open))

(event Custom|Event%20LockMissing
  (CallFunction|UpdateAngle (Variables|Default|GetOpenAngle)))

(event EventBeginPlay
  (bind _lockref (Variables|Default|GetLockRef))
  (|CallParentFunction)
  (EventDispatchers|BindEventtoUnlocked _lockref (delegate Custom|Event%20Open))
  (EventDispatchers|BindEventtoDestroyed _lockref (delegate Custom|Event%20LockMissing)))

(event Collision|EventActorBeginOverlap
  (params (OtherActor :type Actor%20Object%20Reference))
  (|CallParentFunction OtherActor) ; This node is disabled and will not be called.\nDrag off pins to build functionality.
)

(event EventTick
  (params (DeltaSeconds :type Float%20%28single-precision%29))
  (|CallParentFunction DeltaSeconds) ; This node is disabled and will not be called.\nDrag off pins to build functionality.
)

(fn ConstructionScript
  (|CallParentFunction))