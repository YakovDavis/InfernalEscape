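; AI controller for the skeleton enemy that runs its behavior tree and tracks the player as its target.
; On possess it seeds the Blackboard with the start position and the pawn's patrol radius.
; Sensing the player, or the skeleton being attacked, sets line of sight and makes the player the enemy.
; Other perception updates start a grace timer that clears both keys on expiry.
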(event OnTargetPerceptionUpdated(AIPerception)
  (params (Actor :type Actor%20Object%20Reference) (Stimulus :type AI%20Stimulus%20Structure))
  (bind _blackboard (Variables|Default|GetBlackboard))
  (if (and (Actor|ActorHasTag Actor "Player") (.bSuccessfullySensed (Utilities|Struct|BreakAIStimulus Stimulus)))
    (Utilities|Time|ClearandInvalidateTimerbyHandle (Variables|Default|GetEnemyTimer))
    (AI|Components|Blackboard|SetValueasBool _blackboard (Variables|Default|GetHasLineOfSight) true)
    (AI|Components|Blackboard|SetValueasObject _blackboard (Variables|Default|GetEnemyActor) (Game|Player|GetPlayerPawn 0))
    (else
      (bind _returnvalue (Utilities|Time|SetTimerbyEvent (delegate Custom|StartEnemyTimer) (Variables|Default|GetLineOfSightTimer)))
      (Variables|Default|SetEnemyTimer _returnvalue))))

(event Custom|Event%20WasAttacked
  (bind _blackboard (Variables|Default|GetBlackboard))
  (Utilities|Time|ClearandInvalidateTimerbyHandle (Variables|Default|GetEnemyTimer))
  (AI|Components|Blackboard|SetValueasBool _blackboard (Variables|Default|GetHasLineOfSight) true)
  (AI|Components|Blackboard|SetValueasObject _blackboard (Variables|Default|GetEnemyActor) (Game|Player|GetPlayerPawn 0)))

(event Custom|StartEnemyTimer
  (bind _blackboard (Variables|Default|GetBlackboard))
  (AI|Components|Blackboard|SetValueasBool _blackboard (Variables|Default|GetHasLineOfSight) false)
  (AI|Components|Blackboard|SetValueasObject _blackboard (Variables|Default|GetEnemyActor) 0))

(event EventPossess
  (params (PossessedPawn :type Pawn%20Object%20Reference))
  (bind _returnvalue (Pawn|GetControlledPawn))
  (bind _blackboard (Variables|Default|GetBlackboard))
  (AI|RunBehaviorTree "/Game/Blueprints/BT_Skeleton.BT_Skeleton")
  (AI|Components|Blackboard|SetValueasVector _blackboard (Variables|Default|GetStartPos) (Transformation|GetActorLocation _returnvalue))
  (bind _asbp_skeleton (Utilities|Casting|CastToBP_Skeleton _returnvalue))
  (AI|Components|Blackboard|SetValueasFloat _blackboard (Variables|Default|GetRadius) (Variables|/Game/Blueprints/BP_Skeleton.BP_Skeleton_C|GetPatrolRadius _asbp_skeleton))
  (EventDispatchers|BindEventtoWasAttacked _asbp_skeleton (delegate Custom|Event%20WasAttacked)))

(fn ConstructionScript)